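; BP_FadeInDelay is a level event that shows a fade-in screen and holds completion until the fade finishes.
; When triggered, it creates a WBP_FadeIn widget for the first player controller and adds it to that player's screen.
; A callback bound to the widget's animation-complete event then reports the event as completed.
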(event `self.TriggerEvent`
  (bind _returnvalue (`|CreateWidget` "/Game/TRPG/Events/ExampleLevelEvents/FadeInEvent/WBP_FadeIn.WBP_FadeIn_C" (`GameplayStatics.GetPlayerController` 0)))
  (`UserWidget.AddToPlayerScreen` _returnvalue 0)
  (add `/Game/TRPG/Events/ExampleLevelEvents/FadeInEvent/WBP_FadeIn.AnimationComplete` _returnvalue (delegate `OnAnimComplete`)))

(event `OnAnimComplete`
  (`self.TriggerEventCompleted`))

(fn `UserConstructionScript`
  (`parent.UserConstructionScript`))