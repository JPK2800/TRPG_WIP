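; BP_ParrySkill is a TRPG skill that gives a unit a chance to reduce the damage of an incoming physical attack.
; Its pre-attacked effect requires a physical target weapon, then reads a stat from the owner's fight stats as a percentage chance.
; A successful random roll activates the skill with a fixed negative flat damage modifier, while every other path returns it inactive with no modifiers.
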(fn `Trigger_PreAttackedEffects`
  (params (OwnerUnit :type "/Game/TRPG/Units/Blueprints/BP_GameUnitBase Object Reference") (TargetUnit :type "/Game/TRPG/Units/Blueprints/BP_GameUnitBase Object Reference") (OwnerWeapon :type "/Game/TRPG/Items/Weapons/BP_EquippableWeaponItem Object Reference") (TargetWeapon :type "/Game/TRPG/Items/Weapons/BP_EquippableWeaponItem Object Reference") (OwnerIsInstigator :type Boolean) (TurnNumber :type Byte) (OwnerFightStats :type "/Game/TRPG/CombatCalculations/Struct_Stats Structure") (EnemyFightStats :type "/Game/TRPG/CombatCalculations/Struct_Stats Structure"))
  (returns (SkillActivated :type Boolean) (FlatDamageModifier :type Integer) (PercentDamageModifier :type Integer))
  (bind (_value _returnvalue) (`BlueprintMapLibrary.Map_Find` (`.StatMap_37_3D6B118B4BA2F688CF156C9CD64A4AEB` (break `/Game/TRPG/CombatCalculations/Struct_Stats` OwnerFightStats)) "NewEnumerator3"))
  (if (`/Game/TRPG/Items/Weapons/BP_EquippableWeaponItem.IsPhysical` TargetWeapon)
    (if _returnvalue
      (if (<= (`KismetMathLibrary.RandomFloatInRange` 0.0 1.0) (/ (`KismetMathLibrary.Conv_ByteToDouble` _value) 100.0))
        (return true -10 0)
        (else
          _))))
  (return false 0 0))