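; Base class for TRPG unit skills, exposing overridable hooks that let a skill affect fights, turns and enemy AI targeting.
; Hooks cover pre-fight passives, attacking, being attacked, post-fight and turn start, receiving context such as units, weapons and fight stats.
; Defaults are inert, reporting no activation, damage modifiers or priority changes.
; The post-fight reset clears the skill's nullified flag, so child overrides must call the parent.
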(fn `EnemyLogic_InfluenceBehavior`
  (returns (HighPriorityTarget :type Boolean) (LowPriorityTarget :type Boolean))
  (return false false))

(fn `PostFight_Effects`
  (params (OwnerUnit :type "/Game/TRPG/Units/Blueprints/BP_GameUnitBase Object Reference") (TargetUnit :type "/Game/TRPG/Units/Blueprints/BP_GameUnitBase Object Reference") (OwnerWeapon :type "/Game/TRPG/Items/Weapons/BP_EquippableWeaponItem Object Reference") (TargetWeapon :type "/Game/TRPG/Items/Weapons/BP_EquippableWeaponItem Object Reference") (OwnerIsInstigator :type Boolean) (TurnNumber :type Byte) (OwnerFightStats :type "/Game/TRPG/CombatCalculations/Struct_Stats Structure") (EnemyFightStats :type "/Game/TRPG/CombatCalculations/Struct_Stats Structure"))
  (returns (SkillActivated :type Boolean))
  (return false))

(fn `PreFight_PassiveEffects`
  (params (OwnerUnit :type "GameUnit Object Reference") (TargetUnit :type "GameUnit Object Reference") (OwnerWeapon :type "/Game/TRPG/Items/Weapons/BP_EquippableWeaponItem Object Reference") (TargetWeapon :type "/Game/TRPG/Items/Weapons/BP_EquippableWeaponItem Object Reference") (IsOwnerInstigated :type Boolean) (TurnNumber :type Byte) (OwnerFightStats :type "/Game/TRPG/CombatCalculations/Struct_Stats Structure") (TargetFightStats :type "/Game/TRPG/CombatCalculations/Struct_Stats Structure"))
  (returns (StatModifiersSelf :type "/Game/TRPG/CombatCalculations/Struct_Stats Structure") (StatModifiersTarget :type "/Game/TRPG/CombatCalculations/Struct_Stats Structure") (NegateTargetModifiers :type Boolean) (NegateOwnModifiers :type Boolean) (MoveFirstPriority :type Boolean) (SkillActivated :type Boolean))
  (return (struct) (struct) false false false false))

(fn `ResetSkillDataPostFight`
  ;[0.309 0.3698 0.2188] Ensure the skill is not nullified after this fight. Make ssure child classes call this parent function.
  (set `self.SkillIsNullifiedForFight` false))

(fn `ResetSkillDataPostTurn`
  (params (EndingTurn :type Byte))
  ;[1 1 1] Implement if this skill logic should change between turns
)

(fn `Trigger_PostAttackedEffects`
  (params (OwnerUnit :type "/Game/TRPG/Units/Blueprints/BP_GameUnitBase Object Reference") (TargetUnit :type "/Game/TRPG/Units/Blueprints/BP_GameUnitBase Object Reference") (OwnerWeapon :type "/Game/TRPG/Items/Weapons/BP_EquippableWeaponItem Object Reference") (TargetWeapon :type "/Game/TRPG/Items/Weapons/BP_EquippableWeaponItem Object Reference") (OwnerIsInstigator :type Boolean) (TurnNumber :type Byte) (OwnerFightStats :type "/Game/TRPG/CombatCalculations/Struct_Stats Structure") (EnemyFightStats :type "/Game/TRPG/CombatCalculations/Struct_Stats Structure"))
  (returns (SkillActivated :type Boolean))
  (return false))

(fn `Trigger_PostAttackEffects`
  (params (OwnerUnit :type "/Game/TRPG/Units/Blueprints/BP_GameUnitBase Object Reference") (TargetUnit :type "/Game/TRPG/Units/Blueprints/BP_GameUnitBase Object Reference") (OwnerWeapon :type "/Game/TRPG/Items/Weapons/BP_EquippableWeaponItem Object Reference") (TargetWeapon :type "/Game/TRPG/Items/Weapons/BP_EquippableWeaponItem Object Reference") (OwnerIsInstigator :type Boolean) (TurnNumber :type Byte) (OwnerFightStats :type "/Game/TRPG/CombatCalculations/Struct_Stats Structure") (EnemyFightStats :type "/Game/TRPG/CombatCalculations/Struct_Stats Structure"))
  (returns (SkillActivated :type Boolean))
  (return false))

(fn `Trigger_PreAttackedEffects`
  (params (OwnerUnit :type "/Game/TRPG/Units/Blueprints/BP_GameUnitBase Object Reference") (TargetUnit :type "/Game/TRPG/Units/Blueprints/BP_GameUnitBase Object Reference") (OwnerWeapon :type "/Game/TRPG/Items/Weapons/BP_EquippableWeaponItem Object Reference") (TargetWeapon :type "/Game/TRPG/Items/Weapons/BP_EquippableWeaponItem Object Reference") (OwnerIsInstigator :type Boolean) (TurnNumber :type Byte) (OwnerFightStats :type "/Game/TRPG/CombatCalculations/Struct_Stats Structure") (EnemyFightStats :type "/Game/TRPG/CombatCalculations/Struct_Stats Structure"))
  (returns (SkillActivated :type Boolean) (FlatDamageModifier :type Integer) (PercentDamageModifier :type Integer))
  (return false 0 0))

(fn `Trigger_PreAttackEffects`
  (params (OwnerUnit :type "/Game/TRPG/Units/Blueprints/BP_GameUnitBase Object Reference") (TargetUnit :type "/Game/TRPG/Units/Blueprints/BP_GameUnitBase Object Reference") (OwnerWeapon :type "/Game/TRPG/Items/Weapons/BP_EquippableWeaponItem Object Reference") (TargetWeapon :type "/Game/TRPG/Items/Weapons/BP_EquippableWeaponItem Object Reference") (OwnerIsInstigator :type Boolean) (TurnNumber :type Byte) (OwnerFightStats :type "/Game/TRPG/CombatCalculations/Struct_Stats Structure") (EnemyFightStats :type "/Game/TRPG/CombatCalculations/Struct_Stats Structure"))
  (returns (SkillActivated :type Boolean) (FlatDamageModifier :type Integer) (PercentDamageModifier :type Integer))
  (return false 0 0))

(fn `Trigger_PreFightEffects`
  (params (OwnerUnit :type "/Game/TRPG/Units/Blueprints/BP_GameUnitBase Object Reference") (TargetUnit :type "/Game/TRPG/Units/Blueprints/BP_GameUnitBase Object Reference") (OwnerWeapon :type "/Game/TRPG/Items/Weapons/BP_EquippableWeaponItem Object Reference") (TargetWeapon :type "/Game/TRPG/Items/Weapons/BP_EquippableWeaponItem Object Reference") (OwnerIsInstigator :type Boolean) (TurnNumber :type Byte) (OwnerFightStats :type "/Game/TRPG/CombatCalculations/Struct_Stats Structure") (TargetFightStats :type "/Game/TRPG/CombatCalculations/Struct_Stats Structure"))
  (returns (SkillActivated :type Boolean))
  (return false))

(fn `TurnStartEffects`
  (params (Owner :type "/Game/TRPG/Units/Blueprints/BP_GameUnitBase Object Reference"))
  (returns (SkillActivated :type Boolean))
  (return false))