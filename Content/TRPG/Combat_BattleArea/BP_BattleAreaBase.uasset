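; Base battle arena actor for TRPG combat, staging an instigator and a responder unit away from their grid tiles.
; Initialization stores both units and precalculated combat data and resets the action phase.
; Units teleport to the arena's start components and return to their saved tile and facing.
; A timer calls "StartFirstAction" by name, which this file lacks; the similarly named StartFirstUnitAction is an empty stub.
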(fn `InitializeBattlePhase`
  (params (InstigatorUnit :type "/Game/TRPG/Units/Blueprints/BP_GameUnitBase Object Reference") (ResponderUnit :type "/Game/TRPG/Units/Blueprints/BP_GameUnitBase Object Reference") (CalculatedCombatData :type "/Game/TRPG/CombatCalculations/Struct_CalculatedCombat Structure"))
  (set `self.CurrentActionPhase` "NewEnumerator0")
  (set `self.InstigatorUnitWorld` InstigatorUnit)
  (set `self.ResponderUnitWorld` ResponderUnit)
  (set `self.CombatData` CalculatedCombatData))

(fn `MoveUnitsBackToTiles`
  (bind _instigatorunitworld (`self.InstigatorUnitWorld`))
  (bind _responderunitworld (`self.ResponderUnitWorld`))
  (`|ExecutionSequence`
    (:`then_0`
      (`GameUnit.SetUnitLocAndRot` _instigatorunitworld (`GameUnit.GetCurrentUnitTile` _instigatorunitworld) (`GameUnit.GetCurrentUnitDirection` _instigatorunitworld)))
    (:`then_1`
      (`GameUnit.SetUnitLocAndRot` _responderunitworld (`GameUnit.GetCurrentUnitTile` _responderunitworld) (`GameUnit.GetCurrentUnitDirection` _responderunitworld)))))

(fn `MoveUnitsToArena`
  (bind _responderstart (`self.ResponderStart`))
  (bind _instigatorstart (`self.InstigatorStart`))
  (`|ExecutionSequence`
    (:`then_0`
      (`self.K2_SetActorLocationAndRotation` (`self.InstigatorUnitWorld`) (`SceneComponent.K2_GetComponentLocation` _instigatorstart) (`SceneComponent.K2_GetComponentRotation` _instigatorstart) false true))
    (:`then_1`
      (`self.K2_SetActorLocationAndRotation` (`self.ResponderUnitWorld`) (`SceneComponent.K2_GetComponentLocation` _responderstart) (`SceneComponent.K2_GetComponentRotation` _responderstart) false true))))

(fn `StartFirstPhaseTimer`
  (`KismetSystemLibrary.K2_SetTimer` null "StartFirstAction" 3.0))

(fn `StartFirstUnitAction`)

(fn `UserConstructionScript`)