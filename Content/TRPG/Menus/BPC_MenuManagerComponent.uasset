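; Actor component that builds and stacks menu widgets for the tactical RPG's units and tiles.
; CreateBasicWidget constructs option objects from classes; CreateActionItemWidget wraps items with usability color and targetable units, plus one itemless entry.
; Both register widgets through AddNewActiveWidget, which uses BPI_MenuInterface to pause the current menu and initialize the new one.
; RemoveActiveWidget closes the active menu and unpauses the stack's last, without reassigning ActiveWidget.
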(fn `AddNewActiveWidget`
  (params (Widget :type "UserWidget Object Reference"))
  (bind _activewidget (`self.ActiveWidget`))
  (if (`KismetSystemLibrary.DoesImplementInterface` Widget "/Game/TRPG/Menus/BPI_MenuInterface.BPI_MenuInterface_C")
    (`|ExecutionSequence`
      (:`then_0`
        (`/Engine/EditorBlueprintResources/StandardMacros.IsValid` _activewidget
          (:`Is Valid`
            (bind _asbpi_menu_interface (cast `/Game/TRPG/Menus/BPI_MenuInterface` _activewidget))
            (`/Game/TRPG/Menus/BPI_MenuInterface.PauseWidget` _asbpi_menu_interface))))
      (:`then_1`
        (`KismetArrayLibrary.Array_Add` (`self.WidgetStack`) Widget)
        (bind _output_get (set `self.ActiveWidget` Widget))
        (`|ExecutionSequence`
          (:`then_0`
            (bind _asbpi_menu_interface_2 (cast `/Game/TRPG/Menus/BPI_MenuInterface` _output_get))
            (`/Game/TRPG/Menus/BPI_MenuInterface.InitializeWidget` _asbpi_menu_interface_2 self)))))
    (else
      (`KismetSystemLibrary.PrintString` (`KismetStringLibrary.Concat_StrStr` (`KismetStringLibrary.Conv_ObjectToString` Widget) " widget does not implement the menu interface!")))))

(fn `CreateActionItemWidget`
  (params (GameItems :type "Array of /Game/TRPG/Items/BP_GameItem Object Reference") (RelevantUnit :type "/Game/TRPG/Units/Blueprints/BP_GameUnitBase Object Reference") (RelevantTile :type "/Game/TRPG/Tiles/Blueprints/BP_GameTile Object Reference") (GameMode :type "/Game/BP_CombatGameMode Object Reference") (GameInstance :type "/Game/BP_GameInstance Object Reference"))
  (returns (ActionWidget :type "/Game/TRPG/Menus/ItemMenuWidgets/WBP_ActionItemMenu Object Reference"))
  (locals (ActionItemObjects :type "Array of /Game/TRPG/Menus/BP_ActionItemMenuObject Object Reference") (ItemObjectToTargets :type "Map of /Game/TRPG/Menus/BP_ActionItemMenuObject Object Reference to /Game/TRPG/Menus/ItemMenuWidgets/Struct_TargetableUnits Structure"))
  (`|ExecutionSequence`
    (:`then_0`
      (for _array_element GameItems
        (bind (_visible _color _targetableunits) (`/Game/TRPG/Menus/BPFL_MenuUtility.Calculate if Item Is Usable` _array_element true RelevantUnit RelevantTile))
        (bind _returnvalue (`|GenericCreateObject` "/Game/TRPG/Menus/BP_ActionItemMenuObject.BP_ActionItemMenuObject_C" _array_element _color RelevantUnit RelevantTile GameMode GameInstance))
        (`KismetArrayLibrary.Array_Add` (`local.ActionItemObjects`) _returnvalue)
        (`BlueprintMapLibrary.Map_Add` (`local.ItemObjectToTargets`) _returnvalue (make `/Game/TRPG/Menus/ItemMenuWidgets/Struct_TargetableUnits` _targetableunits))))
    (:`then_1`
      (bind _returnvalue_2 (`|GenericCreateObject` "/Game/TRPG/Menus/BP_ActionItemMenuObject.BP_ActionItemMenuObject_C" null "NewEnumerator1" RelevantUnit RelevantTile GameMode GameInstance))
      (`KismetArrayLibrary.Array_Add` (`local.ActionItemObjects`) _returnvalue_2))
    (:`then_2`
      (bind _returnvalue_3 (`|CreateWidget` "/Game/TRPG/Menus/ItemMenuWidgets/WBP_ActionItemMenu.WBP_ActionItemMenu_C" (`GameplayStatics.GetPlayerController` 0) (`local.ActionItemObjects`) (0.0 0.0) (`local.ItemObjectToTargets`)))
      (`|ExecutionSequence`
        (:`then_0`
          (bind _asbpi_menu_interface (cast `/Game/TRPG/Menus/BPI_MenuInterface` _returnvalue_3))
          (`/Game/TRPG/Menus/BPI_MenuInterface.InitializeWidget` _asbpi_menu_interface self))
        (:`then_1`
          (`self.AddNewActiveWidget` _returnvalue_3)
          (`UserWidget.AddToPlayerScreen` _returnvalue_3 0)
          (return _returnvalue_3))))))

(fn `CreateBasicWidget`
  (params (MenuObjects :type "Array of /Game/TRPG/Menus/BP_MenuObject Class Reference") (RelevantUnit :type "/Game/TRPG/Units/Blueprints/BP_GameUnitBase Object Reference") (RelevantTile :type "/Game/TRPG/Tiles/Blueprints/BP_GameTile Object Reference") (GameMode :type "/Game/BP_CombatGameMode Object Reference") (GameInstance :type "/Game/BP_GameInstance Object Reference"))
  (returns (Menu :type "/Game/TRPG/Menus/MenuWidgets/WBP_Menu Object Reference"))
  (locals (MenuOptions :type "Array of /Game/TRPG/Menus/BP_MenuObject Object Reference"))
  (`|ExecutionSequence`
    (:`then_0`
      (for _array_element MenuObjects
        (bind _returnvalue (`|GenericCreateObject` _array_element RelevantUnit RelevantTile GameMode GameInstance))
        (`KismetArrayLibrary.Array_Add` (`local.MenuOptions`) _returnvalue)))
    (:`then_1`
      (bind _returnvalue_2 (`|CreateWidget` "/Game/TRPG/Menus/MenuWidgets/WBP_Menu.WBP_Menu_C" (`GameplayStatics.GetPlayerController` 0) (`local.MenuOptions`)))
      (`|ExecutionSequence`
        (:`then_0`
          (bind _asbpi_menu_interface (cast `/Game/TRPG/Menus/BPI_MenuInterface` _returnvalue_2))
          (`/Game/TRPG/Menus/BPI_MenuInterface.InitializeWidget` _asbpi_menu_interface self))
        (:`then_1`
          (`self.AddNewActiveWidget` _returnvalue_2)
          (`UserWidget.AddToPlayerScreen` _returnvalue_2 0)
          (return _returnvalue_2))))))

(fn `RemoveActiveWidget`
  (bind _activewidget (`self.ActiveWidget`))
  (bind _widgetstack (`self.WidgetStack`))
  (bind _output (`|GetArrayItem` _widgetstack (`KismetArrayLibrary.Array_LastIndex` _widgetstack)))
  (`/Engine/EditorBlueprintResources/StandardMacros.IsValid` _activewidget
    (:`Is Valid`
      (`KismetArrayLibrary.Array_RemoveItem` (`self.WidgetStack`) _activewidget)
      (bind _asbpi_menu_interface (cast `/Game/TRPG/Menus/BPI_MenuInterface` _activewidget))
      (`/Game/TRPG/Menus/BPI_MenuInterface.CloseAndDestroyWidget` _asbpi_menu_interface)
      (`/Engine/EditorBlueprintResources/StandardMacros.IsValid` _output
        (:`Is Valid`
          (bind _asbpi_menu_interface_2 (cast `/Game/TRPG/Menus/BPI_MenuInterface` _output))
          (`/Game/TRPG/Menus/BPI_MenuInterface.UnpauseWidget` _asbpi_menu_interface_2))))))