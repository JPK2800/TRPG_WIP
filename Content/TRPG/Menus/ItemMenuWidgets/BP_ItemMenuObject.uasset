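; BP_ItemMenuObject is a menu option object for items in the TRPG menus, handling what happens when the option is triggered.
; TriggerOption runs the parent behavior, then, for unit action items, expects the menu to be a WBP_AttackItemMenu.
; It looks itself up in that menu's TargetableUnits map, puts the control pawn into unit targeting with the mapped units and closes the menu.
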(fn `TriggerOption`
  (params (GameMode :type "/Game/BP_CombatGameMode Object Reference") (MenuWidget :type "Object Object Reference"))
  (`parent.TriggerOption` GameMode MenuWidget)
  (if (`self.IsUnitActionItem`)
    (bind _aswbp_item_menu (cast `/Game/TRPG/Menus/ItemMenuWidgets/WBP_AttackItemMenu` MenuWidget))
    (bind (_value _returnvalue) (`BlueprintMapLibrary.Map_Find` (`/Game/TRPG/Menus/ItemMenuWidgets/WBP_AttackItemMenu.TargetableUnits` _aswbp_item_menu) self))
    (if _returnvalue
      (bind _returnvalue_2 (`CombatGameMode.GetControlPawn` GameMode))
      (`TileControlPawn.SetUnitTargetingPhase` _returnvalue_2 (`.Units_4_BE7677454CC2C4FA4F9AD4B35B89A6C3` (break `/Game/TRPG/Menus/ItemMenuWidgets/Struct_TargetableUnits` _value)))
      (`/Game/TRPG/Menus/ItemMenuWidgets/WBP_AttackItemMenu.CloseWidget` _aswbp_item_menu))))