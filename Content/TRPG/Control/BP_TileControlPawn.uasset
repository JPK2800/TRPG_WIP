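; Player pawn for a tile-based tactics game that turns tile hover, movement and targeting events into UI and selected-unit feedback.
; Hovering glides a marker to the tile with VInterpTo on Tick and refreshes terrain and unit info widgets.
; Movement events toggle run/idle animations through an interface, and targeting snaps unit facing by look-at yaw quadrant.
; It also opens the unit action and inventory menus and triggers pre-combat calculations.
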(event `self.ReceiveBeginPlay`
  (add `self.OnTileHover` (delegate `OnTileHover_Event`))
  (add `self.OnTileMovementConfirm` (delegate `OnTileMovementConfirm_Event`))
  (add `self.OnCancelUnitMovementAndAction` (delegate `EndUnitMovementAndAction_Event`))
  (add `self.OnTileMovementComplete` (delegate `EndUnitMovementAndAction_Event`))
  (add `self.OnCancelTargetingUnits` (delegate `OnCancelTargetingUnits_Event`))
  (add `self.OnTargetTile` (delegate `OnTargetTile_Event`))
  (add `self.OnCancelTargetingUnits` (delegate `OnCancelTargetTile_Event`)))

(event `OnTargetTile_Event` :!signature `self.OnTargetTile`
  (params (Unit :type "GameUnit Object Reference"))
  (`self.UnitFaceTowardsTarget` Unit))

(event `OnTileHover_Event` :!signature `self.OnTileHover`
  (params (Tile :type "GameTile Object Reference"))
  (`self.MoveHoverWidgetToHoverTile`)
  (`self.UpdateTileInfoWidget` Tile)
  (`self.DisplayUnitData` Tile))

(event `OnTileMovementConfirm_Event`
  (`self.SetSelectedUnitMoving`))

(event `EndUnitMovementAndAction_Event`
  (`self.SetSelectedUnitIdle`))

(event `OnCancelTargetingUnits_Event`
  (`self.RedisplayUnitInventoryWidget`))

(event `OnCancelTargetTile_Event`
  (`self.UnitFaceTowardsTarget` null))

(event `self.ReceiveTick`
  (params (DeltaSeconds :type "Float (single-precision)"))
  (`self.MoveHoverWidgetStep` DeltaSeconds))

(event `self.UnitReadyForActions`
  (params (Unit :type "GameUnit Object Reference") (Tile :type "GameTile Object Reference"))
  (bind (_targetdir _returnvalue) (`self.GetUnitDestinationTile`))
  (bind _asbp_game_unit_base (cast `/Game/TRPG/Units/Blueprints/BP_GameUnitBase` Unit))
  (`GameUnit.SetUnitLocAndRot` _asbp_game_unit_base _returnvalue _targetdir)
  (bind _asbp_game_tile (cast `/Game/TRPG/Tiles/Blueprints/BP_GameTile` Tile))
  (`self.DisplayUnitActionMenuWidget` _asbp_game_unit_base _asbp_game_tile))

(fn `DisplayPreCombatCalculations`
  (params (TargetGameUnit :type "GameUnit Object Reference"))
  (bind _asbp_game_unit_base (cast `/Game/TRPG/Units/Blueprints/BP_GameUnitBase` TargetGameUnit))
  (bind _asbp_game_unit_base_2 (cast `/Game/TRPG/Units/Blueprints/BP_GameUnitBase` (`self.SelectedUnit`)))
  (bind (_founddata _weapon) (`/Game/TRPG/Units/Blueprints/BP_GameUnitBase.GetEquippedItemOfType` _asbp_game_unit_base "Weapon"))
  (bind (_founddata_2 _weapon_2) (`/Game/TRPG/Units/Blueprints/BP_GameUnitBase.GetEquippedItemOfType` _asbp_game_unit_base_2 "Weapon"))
  (`/Game/TRPG/CombatCalculations/BPFL_CombatCalculations.PreCombatCalculation` _weapon_2 _weapon _asbp_game_unit_base_2 _asbp_game_unit_base))

(fn `DisplayUnitActionMenuWidget`
  (params (Unit :type "/Game/TRPG/Units/Blueprints/BP_GameUnitBase Object Reference") (Tile :type "/Game/TRPG/Tiles/Blueprints/BP_GameTile Object Reference"))
  (locals (MenuOptions :type "Array of /Game/TRPG/Menus/MenuWidgets/BP_MenuObject Object Reference"))
  (bind _menu (`/Game/TRPG/Menus/BPFL_MenuUtility.CreateBasicMenu` (`|MakeArray` "/Game/TRPG/Menus/UnitTurnOptions/BP_UnitTurnAttack.BP_UnitTurnAttack_C" "/Game/TRPG/Menus/UnitTurnOptions/BP_UnitTurnWait.BP_UnitTurnWait_C" "/Game/TRPG/Menus/UnitTurnOptions/BP_UnitTurnCancel.BP_UnitTurnCancel_C" :!type "/Game/TRPG/Menus/MenuWidgets/BP_MenuObject Class Reference") Unit Tile (384.0 0.0)))
  (set `self.UnitTurnWidget` _menu))

(fn `DisplayUnitData`
  (params (Tile :type "GameTile Object Reference"))
  (bind _unitinfowidget (`self.UnitInfoWidget`))
  (bind _currentzoomlevel (`self.CurrentZoomLevel`))
  (bind _unitinfowidget_2 (`self.UnitInfoWidget`))
  (bind _unitinfowidget_3 (`self.UnitInfoWidget`))
  (bind _asbp_game_tile (cast `/Game/TRPG/Tiles/Blueprints/BP_GameTile` Tile))
  (bind (_unit _returnvalue) (`GameTile.GetUnitOnTile` _asbp_game_tile))
  (if _returnvalue
    (bind _asbp_game_unit_base (cast `/Game/TRPG/Units/Blueprints/BP_GameUnitBase` _unit))
    (bind (_founddata _weapon) (`/Game/TRPG/Units/Blueprints/BP_GameUnitBase.GetEquippedItemOfType` _asbp_game_unit_base "Weapon"))
    (if _founddata
      (bind _returnvalue_2 (`|CreateWidget` "/Game/TRPG/Units/UnitHoverDisplay/WBP_UnitHover.WBP_UnitHover_C" (`GameplayStatics.GetPlayerController` 0)))
      (bind _returnvalue_3 (`KismetStringLibrary.Conv_NameToString` (`/Game/TRPG/Units/Blueprints/BP_GameUnitBase.UnitName` _asbp_game_unit_base)))
      (bind _unitleveldata_currentlevel (break `/Game/TRPG/Units/Levels/Struct_LevelData` (`/Game/TRPG/Units/Blueprints/BP_GameUnitBase.UnitLevelData` _asbp_game_unit_base)))
      (bind _hpremaining (`/Game/TRPG/Units/Blueprints/BP_GameUnitBase.HpRemaining` _asbp_game_unit_base))
      (bind (_unitstats_statmap _unitstats_hp) (break `/Game/TRPG/CombatCalculations/Struct_Stats` (`/Game/TRPG/Units/Blueprints/BP_GameUnitBase.UnitStats` _asbp_game_unit_base)))
      (bind _portraiticon (`/Game/TRPG/Units/Blueprints/BP_GameUnitBase.PortraitIcon` _asbp_game_unit_base))
      (bind _returnvalue_4 (cast `EUnitFaction` (`GameUnit.UnitFaction` _asbp_game_unit_base)))
      (`/Game/TRPG/Units/UnitHoverDisplay/WBP_UnitHover.UpdateData` _returnvalue_2 _returnvalue_3 _unitleveldata_currentlevel _hpremaining _unitstats_hp (`KismetStringLibrary.Conv_NameToString` (`InventoryItem.DisplayName` _weapon)) _portraiticon (`/Game/TRPG/Items/BP_GameItem.Icon` _weapon) _returnvalue_4 _asbp_game_unit_base _currentzoomlevel)
      (`/Game/TRPG/Units/UnitHoverDisplay/WBP_UnitHover.BindToTileControlPawn` _returnvalue_2 self)
      (`/Engine/EditorBlueprintResources/StandardMacros.IsValid` _unitinfowidget_3
        (:`Is Valid`
          (`Widget.RemoveFromParent` _unitinfowidget_3))
        (:`Is Not Valid`
          _))
      (bind _output_get (set `self.UnitInfoWidget` _returnvalue_2))
      (`UserWidget.AddToPlayerScreen` _output_get 0)
      (else
        (bind _returnvalue_5 (`|CreateWidget` "/Game/TRPG/Units/UnitHoverDisplay/WBP_UnitHover.WBP_UnitHover_C" (`GameplayStatics.GetPlayerController` 0)))
        (`/Game/TRPG/Units/UnitHoverDisplay/WBP_UnitHover.UpdateData` _returnvalue_5 _returnvalue_3 _unitleveldata_currentlevel _hpremaining _unitstats_hp "" _portraiticon null _returnvalue_4 _asbp_game_unit_base _currentzoomlevel)
        (`/Game/TRPG/Units/UnitHoverDisplay/WBP_UnitHover.BindToTileControlPawn` _returnvalue_5 self)
        (`/Engine/EditorBlueprintResources/StandardMacros.IsValid` _unitinfowidget_2
          (:`Is Valid`
            (`Widget.RemoveFromParent` _unitinfowidget_2))
          (:`Is Not Valid`
            _))
        (bind _output_get_2 (set `self.UnitInfoWidget` _returnvalue_5))
        (`UserWidget.AddToPlayerScreen` _output_get_2 0)))
    (else
      (`/Engine/EditorBlueprintResources/StandardMacros.IsValid` _unitinfowidget
        (:`Is Valid`
          (`Widget.RemoveFromParent` _unitinfowidget))))))

(fn `DisplayUnitInventoryWidget`
  (params (Unit :type "/Game/TRPG/Units/Blueprints/BP_GameUnitBase Object Reference") (Tile :type "/Game/TRPG/Tiles/Blueprints/BP_GameTile Object Reference") (OnlyEnableWeapons :type Boolean))
  (set `self.PrevUnitInventoryIsItemAction` OnlyEnableWeapons)
  (bind _menu (`/Game/TRPG/Menus/BPFL_MenuUtility.CreateItemMenu` (`/Game/TRPG/Units/Blueprints/BP_GameUnitBase.GetUnitInventory` Unit) Unit Tile (0.0 0.0) OnlyEnableWeapons))
  (set `self.UnitInventorySelectionWidget` _menu))

(fn `MoveHoverWidgetStep`
  (params (DeltaTime :type "Float (double-precision)"))
  (bind _hoverwidget (`self.HoverWidget`))
  (bind _hoverwidgettargetloc (`self.HoverWidgetTargetLoc`))
  (bind _returnvalue (`SceneComponent.K2_GetComponentLocation` _hoverwidget))
  (if (`self.MovingHoverWidget`)
    (`SceneComponent.K2_SetWorldLocation` _hoverwidget (`KismetMathLibrary.VInterpTo` _returnvalue _hoverwidgettargetloc DeltaTime 15.0) false false)
    (if (< (`KismetMathLibrary.Vector_Distance` _returnvalue _hoverwidgettargetloc) 3.0)
      (`SceneComponent.K2_SetWorldLocation` _hoverwidget _hoverwidgettargetloc false false)
      (set `self.MovingHoverWidget` false))))

(fn `MoveHoverWidgetToHoverTile`
  (bind _hoverwidget (`self.HoverWidget`))
  (bind _returnvalue (`self.GetHoverTile`))
  (`/Engine/EditorBlueprintResources/StandardMacros.IsValid` _returnvalue
    (:`Is Valid`
      (`SceneComponent.SetHiddenInGame` _hoverwidget false false)
      (set `self.HoverWidgetTargetLoc` (+ (`SceneComponent.K2_GetComponentLocation` (`GameTile.UnitPositionComponent` _returnvalue)) (0.0 0.0 5.0)))
      (set `self.MovingHoverWidget` true)
      (set `SceneComponent.bAbsoluteLocation` true (`self.HoverWidget`)))
    (:`Is Not Valid`
      (`SceneComponent.SetHiddenInGame` _hoverwidget true false))))

(fn `RedisplayUnitInventoryWidget`
  (bind (_targetdir _returnvalue) (`self.GetUnitDestinationTile`))
  (bind _asbp_game_tile (cast `/Game/TRPG/Tiles/Blueprints/BP_GameTile` _returnvalue))
  (bind _asbp_game_unit_base (cast `/Game/TRPG/Units/Blueprints/BP_GameUnitBase` (`self.SelectedUnit`)))
  (`self.DisplayUnitInventoryWidget` _asbp_game_unit_base _asbp_game_tile (`self.PrevUnitInventoryIsItemAction`)))

(fn `RemoveUnitInventoryWidget`
  (`/Engine/EditorBlueprintResources/StandardMacros.IsValid` (`self.UnitInventorySelectionWidget`)))

(fn `SetSelectedUnitIdle`
  (bind _asbp_game_unit (cast `/Game/TRPG/Units/Blueprints/BP_GameUnit` (`self.SelectedUnit`)))
  (bind _returnvalue (`SkeletalMeshComponent.GetAnimInstance` (`/Game/TRPG/Units/Blueprints/BP_GameUnit_3D.BodyMesh` _asbp_game_unit)))
  (`/Engine/EditorBlueprintResources/StandardMacros.IsValid` _returnvalue
    (:`Is Valid`
      (if (`KismetSystemLibrary.DoesImplementInterface` _returnvalue "/Script/TRPG.IUnitAnimations")
        (message `IUnitAnimations.SetIdle` _returnvalue)))))

(fn `SetSelectedUnitMoving`
  (bind _asbp_game_unit (cast `/Game/TRPG/Units/Blueprints/BP_GameUnit` (`self.SelectedUnit`)))
  (bind _returnvalue (`SkeletalMeshComponent.GetAnimInstance` (`/Game/TRPG/Units/Blueprints/BP_GameUnit_3D.BodyMesh` _asbp_game_unit)))
  (`/Engine/EditorBlueprintResources/StandardMacros.IsValid` _returnvalue
    (:`Is Valid`
      (if (`KismetSystemLibrary.DoesImplementInterface` _returnvalue "/Script/TRPG.IUnitAnimations")
        (message `IUnitAnimations.SetRun` _returnvalue)))))

(fn `UnitFaceTowardsTarget`
  (params (TargetUnit :type "GameUnit Object Reference"))
  (returns (NewDir :type "ECardinalDirections Enum"))
  (locals (LocalYaw :type "Float (single-precision)" :default 0.0))
  (bind _selectedunit (`self.SelectedUnit`))
  (bind _selectedunit_2 (`self.SelectedUnit`))
  (bind _selectedunit_3 (`self.SelectedUnit`))
  (bind _localyaw (`local.LocalYaw`))
  (bind _localyaw_2 (`local.LocalYaw`))
  (`/Engine/EditorBlueprintResources/StandardMacros.IsValid` _selectedunit_2
    (:`Is Valid`
      (`/Engine/EditorBlueprintResources/StandardMacros.IsValid` TargetUnit
        (:`Is Valid`
          (set `local.LocalYaw` (.yaw (`KismetMathLibrary.FindLookAtRotation` (`self.K2_GetActorLocation` _selectedunit_2) (`self.K2_GetActorLocation` TargetUnit))))
          (`|ExecutionSequence`
            (:`then_0`
              (if (< _localyaw 0.0)
                (set `local.LocalYaw` (+ _localyaw 360.0))))
            (:`then_1`
              (`|ExecutionSequence`
                (:`then_0`
                  (if (or (< _localyaw_2 45.0) (> _localyaw_2 315.0))
                    (`GameUnit.SetCurrentUnitDirection` _selectedunit_3 "UP_DIR")
                    (return "UP_DIR")))
                (:`then_1`
                  (if (<= _localyaw_2 135.0)
                    (`GameUnit.SetCurrentUnitDirection` _selectedunit_3 "RIGHT_DIR")
                    (return "RIGHT_DIR")))
                (:`then_2`
                  (if (< _localyaw_2 225.0)
                    (`GameUnit.SetCurrentUnitDirection` _selectedunit "DOWN_DIR")
                    (return "DOWN_DIR")
                    (else
                      (`GameUnit.SetCurrentUnitDirection` _selectedunit "LEFT_DIR")
                      (return "LEFT_DIR"))))))))
        (:`Is Not Valid`
          (bind _targetdir (`self.GetUnitDestinationTile`))
          (`GameUnit.SetCurrentUnitDirection` _selectedunit_2 _targetdir))))))

(fn `UpdateTileInfoWidget`
  (params (HoveredTile :type "GameTile Object Reference"))
  (bind _asbp_game_tile (cast `/Game/TRPG/Tiles/Blueprints/BP_GameTile` HoveredTile))
  (`/Engine/EditorBlueprintResources/StandardMacros.IsValid` _asbp_game_tile
    (:`Is Valid`
      (`/Engine/EditorBlueprintResources/StandardMacros.IsValid` (`self.TileInfoWidget`)
        (:`Is Valid`
          _)
        (:`Is Not Valid`
          (bind _returnvalue (`|CreateWidget` "/Game/TRPG/Tiles/DisplayTileInfo/WBP_Tile_Info_Widget.WBP_Tile_Info_Widget_C" (`GameplayStatics.GetPlayerController` 0)))
          (`UserWidget.AddToPlayerScreen` _returnvalue 0)
          (set `self.TileInfoWidget` _returnvalue)))
      (`/Game/TRPG/Tiles/DisplayTileInfo/WBP_Tile_Info_Widget.LoadTerrainInfo` (`self.TileInfoWidget`) (`/Game/TRPG/Tiles/BlueprintFunctions/BPFL_DefaultTerrainData.GetTerrainHudInfo` (`/Game/TRPG/Tiles/Blueprints/BP_GameTile.TileType` _asbp_game_tile))))
    (:`Is Not Valid`
      (`/Engine/EditorBlueprintResources/StandardMacros.IsValid` (`self.TileInfoWidget`)
        (:`Is Valid`
          (`Widget.RemoveFromParent` (`self.TileInfoWidget`)))))))

(fn `UserConstructionScript`)