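; Player controller for a tactical RPG that handles input, combat phase banners and battle menus.
; It registers the Enhanced Input mapping context, forwards actions to Trigger functions, and can save key remaps through user settings.
; Phase changes open either a colored transition banner or the pre-battle menu.
; Menus are WBP_Menu widgets fed constructed option objects, with unit-turn options filtered by visibility checks on unit and tile.
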(event `self.ReceiveBeginPlay`
  (`self.InitInputSystem`))

(event `self.DisplayPhaseChange`
  (params (NewPhase :type "ECombatPhase Enum" :default "NO_PHASE"))
  (`self.DisplayPhaseChangeUi` NewPhase))

(event `EnhancedInput|/Game/TRPG/Control/Inputs/IA_CursorUp`
  (params (ActionValue :type Boolean) (ElapsedSeconds :type "Float (double-precision)") (TriggeredSeconds :type "Float (double-precision)") (InputAction :type "InputAction Object Reference" :default "/Game/TRPG/Control/Inputs/IA_CursorUp.IA_CursorUp"))
  ;[0.3021 0.3021 0.3021] Cursor/Directional Input
  (:`Triggered`
    (`self.TriggerUp`)))

(event `EnhancedInput|/Game/TRPG/Control/Inputs/IA_CursorDown`
  (params (ActionValue :type Boolean) (ElapsedSeconds :type "Float (double-precision)") (TriggeredSeconds :type "Float (double-precision)") (InputAction :type "InputAction Object Reference" :default "/Game/TRPG/Control/Inputs/IA_CursorDown.IA_CursorDown"))
  ;[0.3021 0.3021 0.3021] Cursor/Directional Input
  (:`Triggered`
    (`self.TriggerDown`)))

(event `EnhancedInput|/Game/TRPG/Control/Inputs/IA_CursorLeft`
  (params (ActionValue :type Boolean) (ElapsedSeconds :type "Float (double-precision)") (TriggeredSeconds :type "Float (double-precision)") (InputAction :type "InputAction Object Reference" :default "/Game/TRPG/Control/Inputs/IA_CursorLeft.IA_CursorLeft"))
  ;[0.3021 0.3021 0.3021] Cursor/Directional Input
  (:`Triggered`
    (`self.TriggerLeft`)))

(event `EnhancedInput|/Game/TRPG/Control/Inputs/IA_CamLeft`
  (params (ActionValue :type Boolean) (ElapsedSeconds :type "Float (double-precision)") (TriggeredSeconds :type "Float (double-precision)") (InputAction :type "InputAction Object Reference" :default "/Game/TRPG/Control/Inputs/IA_CamLeft.IA_CamLeft"))
  ;[0.4219 0.4219 0.4219] Camera Directions
  (:`Triggered`
    (`self.TriggerCamLeft`)))

(event `EnhancedInput|/Game/TRPG/Control/Inputs/IA_CursorRight`
  (params (ActionValue :type Boolean) (ElapsedSeconds :type "Float (double-precision)") (TriggeredSeconds :type "Float (double-precision)") (InputAction :type "InputAction Object Reference" :default "/Game/TRPG/Control/Inputs/IA_CursorRight.IA_CursorRight"))
  ;[0.3021 0.3021 0.3021] Cursor/Directional Input
  (:`Triggered`
    (`self.TriggerRight`)))

(event `EnhancedInput|/Game/TRPG/Control/Inputs/IA_CamRight`
  (params (ActionValue :type Boolean) (ElapsedSeconds :type "Float (double-precision)") (TriggeredSeconds :type "Float (double-precision)") (InputAction :type "InputAction Object Reference" :default "/Game/TRPG/Control/Inputs/IA_CamRight.IA_CamRight"))
  ;[0.4219 0.4219 0.4219] Camera Directions
  (:`Triggered`
    (`self.TriggerCamRight`)))

(event `EnhancedInput|/Game/TRPG/Control/Inputs/IA_Confirm`
  (params (ActionValue :type Boolean) (ElapsedSeconds :type "Float (double-precision)") (TriggeredSeconds :type "Float (double-precision)") (InputAction :type "InputAction Object Reference" :default "/Game/TRPG/Control/Inputs/IA_Confirm.IA_Confirm"))
  ;[0.3594 0.3594 0.3594] General Buttons
  (:`Triggered`
    (`self.TriggerConfirm`)))

(event `EnhancedInput|/Game/TRPG/Control/Inputs/IA_CamUp`
  (params (ActionValue :type Boolean) (ElapsedSeconds :type "Float (double-precision)") (TriggeredSeconds :type "Float (double-precision)") (InputAction :type "InputAction Object Reference" :default "/Game/TRPG/Control/Inputs/IA_CamUp.IA_CamUp"))
  ;[0.4219 0.4219 0.4219] Camera Directions
  (:`Triggered`
    (`self.TriggerCamUp`)))

(event `EnhancedInput|/Game/TRPG/Control/Inputs/IA_Cancel`
  (params (ActionValue :type Boolean) (ElapsedSeconds :type "Float (double-precision)") (TriggeredSeconds :type "Float (double-precision)") (InputAction :type "InputAction Object Reference" :default "/Game/TRPG/Control/Inputs/IA_Cancel.IA_Cancel"))
  ;[0.3594 0.3594 0.3594] General Buttons
  (:`Triggered`
    (`self.TriggerCancel`)))

(event `EnhancedInput|/Game/TRPG/Control/Inputs/IA_CamDown`
  (params (ActionValue :type Boolean) (ElapsedSeconds :type "Float (double-precision)") (TriggeredSeconds :type "Float (double-precision)") (InputAction :type "InputAction Object Reference" :default "/Game/TRPG/Control/Inputs/IA_CamDown.IA_CamDown"))
  ;[0.4219 0.4219 0.4219] Camera Directions
  (:`Triggered`
    (`self.TriggerCamDown`)))

(event `EnhancedInput|/Game/TRPG/Control/Inputs/IA_NextUnit`
  (params (ActionValue :type Boolean) (ElapsedSeconds :type "Float (double-precision)") (TriggeredSeconds :type "Float (double-precision)") (InputAction :type "InputAction Object Reference" :default "/Game/TRPG/Control/Inputs/IA_NextUnit.IA_NextUnit"))
  ;[0.3594 0.3594 0.3594] General Buttons
  (:`Triggered`
    (`self.TriggerNextUnit`)))

(event `EnhancedInput|/Game/TRPG/Control/Inputs/IA_MoreInfo`
  (params (ActionValue :type Boolean) (ElapsedSeconds :type "Float (double-precision)") (TriggeredSeconds :type "Float (double-precision)") (InputAction :type "InputAction Object Reference" :default "/Game/TRPG/Control/Inputs/IA_MoreInfo.IA_MoreInfo"))
  ;[0.3594 0.3594 0.3594] General Buttons
  (:`Triggered`
    (`self.TriggerMoreInfo`)))

(event `EnhancedInput|/Game/TRPG/Control/Inputs/IA_MapPress`
  (params (ActionValue :type Boolean) (ElapsedSeconds :type "Float (double-precision)") (TriggeredSeconds :type "Float (double-precision)") (InputAction :type "InputAction Object Reference" :default "/Game/TRPG/Control/Inputs/IA_MapPress.IA_MapPress"))
  ;[0.3594 0.3594 0.3594] General Buttons
  (:`Triggered`
    (`self.TriggerMapPress`)))

(event `EnhancedInput|/Game/TRPG/Control/Inputs/IA_ToggleDisplay`
  (params (ActionValue :type Boolean) (ElapsedSeconds :type "Float (double-precision)") (TriggeredSeconds :type "Float (double-precision)") (InputAction :type "InputAction Object Reference" :default "/Game/TRPG/Control/Inputs/IA_ToggleDisplay.IA_ToggleDisplay"))
  ;[0.3594 0.3594 0.3594] General Buttons
  (:`Triggered`
    (`self.TriggerToggleDisplay`)))

(event `EnhancedInput|/Game/TRPG/Control/Inputs/IA_Menu`
  (params (ActionValue :type Boolean) (ElapsedSeconds :type "Float (double-precision)") (TriggeredSeconds :type "Float (double-precision)") (InputAction :type "InputAction Object Reference" :default "/Game/TRPG/Control/Inputs/IA_Menu.IA_Menu"))
  ;[0.3594 0.3594 0.3594] General Buttons
  (:`Triggered`
    (`self.TriggerMenu`)))

(fn `ChangeInputSetting`
  (params (Key :type "Key Structure" :default "None") (InputActionName :type Name))
  (`EnhancedInputUserSettings.MapPlayerKey` (`self.UserInputSettings`) (make `MapPlayerKeyArgs` InputActionName "Unspecified" Key))
  (`EnhancedInputUserSettings.ApplySettings` (`self.UserInputSettings`))
  (`EnhancedInputUserSettings.SaveSettings` (`self.UserInputSettings`)))

(fn `ClosePreBattleWidget`
  (`Widget.RemoveFromParent` (`self.PreBattleWidget`)))

(fn `DisplayPhaseChangeUi`
  (params (CombatPhase :type "ECombatPhase Enum" :default "NO_PHASE"))
  (switch `ECombatPhase` CombatPhase
    (:`BEFORE_COMBAT`
      (`self.OpenPreBattleWidget`))
    (:`TRANSITION_PLAYER_PHASE`
      (bind _returnvalue (`|CreateWidget` "/Game/TRPG/GeneralDisplay/MenuTransition/WBP_PhaseTransition.WBP_PhaseTransition_C" self "PLAYER PHASE" (struct :`G` 0.193892 :`B` 1.0 :`A` 1.0)))
      (`UserWidget.AddToPlayerScreen` _returnvalue 0))
    (:`TRANSITION_PARTNER_PHASE`
      (bind _returnvalue_2 (`|CreateWidget` "/Game/TRPG/GeneralDisplay/MenuTransition/WBP_PhaseTransition.WBP_PhaseTransition_C" self "ALLY PHASE" (struct :`R` 0.07265 :`G` 1.0 :`A` 1.0)))
      (`UserWidget.AddToPlayerScreen` _returnvalue_2 0))
    (:`TRANSITION_ENEMY_PHASE`
      (bind _returnvalue_3 (`|CreateWidget` "/Game/TRPG/GeneralDisplay/MenuTransition/WBP_PhaseTransition.WBP_PhaseTransition_C" self "ENEMY PHASE" (struct :`R` 1.0 :`B` 0.034709 :`A` 1.0)))
      (`UserWidget.AddToPlayerScreen` _returnvalue_3 0))
    (:`TRANSITION_NPC_PHASE`
      (bind _returnvalue_4 (`|CreateWidget` "/Game/TRPG/GeneralDisplay/MenuTransition/WBP_PhaseTransition.WBP_PhaseTransition_C" self "NEUTRAL PHASE" (struct :`R` 1.0 :`G` 0.974048 :`A` 1.0)))
      (`UserWidget.AddToPlayerScreen` _returnvalue_4 0))))

(fn `DisplayUnitTurnWidget`
  (params (Unit :type "/Game/TRPG/Units/Blueprints/BP_GameUnitBase Object Reference") (Tile :type "/Game/TRPG/Tiles/Blueprints/BP_GameTile Object Reference"))
  (locals (MenuOptions :type "Array of /Game/TRPG/Menus/MenuWidgets/BP_MenuObject Object Reference"))
  (bind _menuoptions (`local.MenuOptions`))
  (`|ExecutionSequence`
    (:`then_0`
      (bind (_visible _color) (`/Game/TRPG/Menus/UnitTurnOptions/BPFL_CalculateIfOptionsIsValid.CalculateIfMenuOptionShouldAppear` "/Game/TRPG/Menus/UnitTurnOptions/BP_UnitTurnAttack.BP_UnitTurnAttack_C" Unit Tile))
      (if _visible
        (bind _returnvalue (`|GenericCreateObject` "/Game/TRPG/Menus/UnitTurnOptions/BP_UnitTurnAttack.BP_UnitTurnAttack_C" _color))
        (`KismetArrayLibrary.Array_Add` _menuoptions _returnvalue)))
    (:`then_1`
      (bind (_visible_2 _color_2) (`/Game/TRPG/Menus/UnitTurnOptions/BPFL_CalculateIfOptionsIsValid.CalculateIfMenuOptionShouldAppear` "/Game/TRPG/Menus/UnitTurnOptions/BP_UnitTurnWait.BP_UnitTurnWait_C" Unit Tile))
      (if _visible_2
        (bind _returnvalue_2 (`|GenericCreateObject` "/Game/TRPG/Menus/UnitTurnOptions/BP_UnitTurnWait.BP_UnitTurnWait_C" _color_2))
        (`KismetArrayLibrary.Array_Add` _menuoptions _returnvalue_2)))
    (:`then_2`
      (bind (_visible_3 _color_3) (`/Game/TRPG/Menus/UnitTurnOptions/BPFL_CalculateIfOptionsIsValid.CalculateIfMenuOptionShouldAppear` "/Game/TRPG/Menus/UnitTurnOptions/BP_UnitTurnWait.BP_UnitTurnWait_C" Unit Tile))
      (if _visible_3
        (bind _returnvalue_3 (`|GenericCreateObject` "/Game/TRPG/Menus/UnitTurnOptions/BP_UnitTurnCancel.BP_UnitTurnCancel_C" _color_3))
        (`KismetArrayLibrary.Array_Add` _menuoptions _returnvalue_3)))
    (:`then_3`
      (bind _returnvalue_4 (`|CreateWidget` "/Game/TRPG/Menus/MenuWidgets/WBP_Menu.WBP_Menu_C" self (`local.MenuOptions`)))
      (set `self.UnitTurnWidget` _returnvalue_4)
      (`/Game/TRPG/Menus/MenuWidgets/WBP_Menu.InitializeOptions` _returnvalue_4)
      (`UserWidget.AddToPlayerScreen` _returnvalue_4 0))))

(fn `InitInputSystem`
  (bind _returnvalue (subsystem `EnhancedInputLocalPlayerSubsystem`))
  (bind _returnvalue_2 (`EnhancedInputSubsystemInterface.GetUserSettings` _returnvalue))
  (`EnhancedInputSubsystemInterface.AddMappingContext` _returnvalue "/Game/TRPG/Control/Inputs/IMC_GameInputs.IMC_GameInputs" 0 (struct))
  (`/Engine/EditorBlueprintResources/StandardMacros.IsValid` _returnvalue_2
    (:`Is Valid`
      (bind _output_get (set `self.UserInputSettings` _returnvalue_2))
      (if (not (`EnhancedInputUserSettings.IsMappingContextRegistered` _output_get "/Game/TRPG/Control/Inputs/IMC_GameInputs.IMC_GameInputs"))
        (`EnhancedInputUserSettings.RegisterInputMappingContext` (`self.UserInputSettings`) "/Game/TRPG/Control/Inputs/IMC_GameInputs.IMC_GameInputs")))))

(fn `OpenPreBattleWidget`
  (bind _returnvalue (`|GenericCreateObject` "/Game/TRPG/Menus/PreBattleOptions/BP_SelectUnits.BP_SelectUnits_C"))
  (bind _returnvalue_2 (`|GenericCreateObject` "/Game/TRPG/Menus/PreBattleOptions/BP_ViewMap.BP_ViewMap_C"))
  (bind _returnvalue_3 (`|GenericCreateObject` "/Game/TRPG/Menus/PreBattleOptions/BP_Inventory.BP_Inventory_C"))
  (bind _returnvalue_4 (`|GenericCreateObject` "/Game/TRPG/Menus/PreBattleOptions/BP_Support.BP_Support_C"))
  (bind _returnvalue_5 (`|GenericCreateObject` "/Game/TRPG/Menus/PreBattleOptions/BP_EquipSkills.BP_EquipSkills_C"))
  (bind _returnvalue_6 (`|GenericCreateObject` "/Game/TRPG/Menus/PreBattleOptions/BP_Save.BP_Save_C"))
  (bind _returnvalue_7 (`|GenericCreateObject` "/Game/TRPG/Menus/PreBattleOptions/BP_Begin.BP_Begin_C"))
  (bind _returnvalue_8 (`|GenericCreateObject` "/Game/TRPG/Menus/PreBattleOptions/BP_Exit.BP_Exit_C"))
  (bind _returnvalue_9 (`|CreateWidget` "/Game/TRPG/Menus/MenuWidgets/WBP_Menu.WBP_Menu_C" self (`|MakeArray` _returnvalue _returnvalue_2 _returnvalue_3 _returnvalue_4 _returnvalue_5 _returnvalue_6 _returnvalue_7 _returnvalue_8 :!type "/Game/TRPG/Menus/MenuWidgets/BP_MenuObject Object Reference")))
  (set `self.PreBattleWidget` _returnvalue_9)
  (`/Game/TRPG/Menus/MenuWidgets/WBP_Menu.InitializeOptions` _returnvalue_9)
  (`UserWidget.AddToPlayerScreen` _returnvalue_9 0))

(fn `UserConstructionScript`)