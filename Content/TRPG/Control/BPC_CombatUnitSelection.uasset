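; Combat unit selection component that loads saved units and spawns them as player-faction units on the map's starting tiles at BeginPlay.
; It loads save slot 0 as a stopgap and reads starting tiles from BP_TileDataActor.
; A sorting pass favors mandatory deployments, compares levels and trims to tile count.
; Spawning ignores that result, walking the unsorted save list by tile index and applying each unit's save and appearance data.
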(event `self.ReceiveBeginPlay`
  (`self.LoadAvailablePreBattleUnits`)
  (`self.LoadTileDataActor`)
  (bind _bestunits (`self.DetermineBestStartingUnits`))
  (bind _output_get (set `self.BestStartingUnits` _bestunits))
  (`self.SpawnUnitsOnTiles` _output_get))

(fn `DetermineBestStartingUnits`
  (returns (BestUnits :type "Array of /Game/TRPG/Units/SaveData/Struct_SaveUnitData Structure"))
  (locals (SortedBattleUnitList :type "Array of /Game/TRPG/Units/SaveData/Struct_SaveUnitData Structure") (CurrentUnitSorted :type Boolean) (MaxPlayerUnitCount :type Integer))
  (bind _tiledata (`self.TileData`))
  (bind _sortedbattleunitlist (`local.SortedBattleUnitList`))
  (bind _sortedbattleunitlist_2 (`local.SortedBattleUnitList`))
  (bind _playerstartingtiles (`TileDataActor.PlayerStartingTiles` _tiledata))
  ;[1 1 1] Get starting tiles for players
  (`/Engine/EditorBlueprintResources/StandardMacros.IsValid` _tiledata
    (:`Is Valid`
      (set `self.StartingTIles` _playerstartingtiles)
      (bind _output_get (set `local.MaxPlayerUnitCount` (`KismetArrayLibrary.Array_Length` _playerstartingtiles)))
      (for _array_element (`self.PreBattleUnitList`)
        (set `local.CurrentUnitSorted` false)
        (bind (_unitname _characterstats _charactermaxstats _leveldata _weaponrankdata _items _skills _unitgameclass _ismandatorydeployment) (break `/Game/TRPG/Units/SaveData/Struct_SaveUnitData` _array_element))
        ;[1 1 1] Prioritize mandatory units
        (if _ismandatorydeployment
          (`KismetArrayLibrary.Array_Insert` (`local.SortedBattleUnitList`) _array_element)
          (set `local.CurrentUnitSorted` true)
          (else
            ;[1 1 1] Insert and sort by level
            (for _index (range (`KismetArrayLibrary.Array_Length` (`local.SortedBattleUnitList`)))
              (if (`KismetArrayLibrary.Array_IsValidIndex` _sortedbattleunitlist_2 _index)
                (if (> (`.CurrentLevel_2_EB3A361F4746CD28D5987CB5D6EACA48` (break `/Game/TRPG/Units/Levels/Struct_LevelData` (`.LevelData_15_E6A0D1734E4600DB79CCF683D7F016C3` (break `/Game/TRPG/Units/SaveData/Struct_SaveUnitData` (`|GetArrayItem` _sortedbattleunitlist_2 _index))))) (`.CurrentLevel_2_EB3A361F4746CD28D5987CB5D6EACA48` (break `/Game/TRPG/Units/Levels/Struct_LevelData` _leveldata)))
                  (`KismetArrayLibrary.Array_Insert` (`local.SortedBattleUnitList`) _array_element _index)
                  (set `local.CurrentUnitSorted` true)
                  (break))))
            ;[1 1 1] ADd to the end of the sorted array if never inserted
            (if (`local.CurrentUnitSorted`)
              (`KismetArrayLibrary.Array_Add` (`local.SortedBattleUnitList`) _array_element)))))
      (`KismetArrayLibrary.Array_Resize` _sortedbattleunitlist _output_get)
      (return _sortedbattleunitlist))))

(fn `LoadAvailablePreBattleUnits`
  (bind _asbp_game_instance (cast `/Game/BP_GameInstance` (`GameplayStatics.GetGameInstance`)))
  ;[1 0 0.05908] TODO: This should be removed with a save-loading menu before the combat map
  (`/Game/BP_GameInstance.LoadSave` _asbp_game_instance 0)
  (bind (_loadeddata _savedata) (`/Game/BP_GameInstance.GetCurrentSaveData` _asbp_game_instance))
  (if _loadeddata
    (set `self.PreBattleUnitList` (`.UnitSaveData_23_88C0CAAE442A39EAE9164DB4A7695BE3` (break `/Game/TRPG/Save/Struct_SaveData` _savedata)))))

(fn `LoadTileDataActor`
  (bind _returnvalue (`GameplayStatics.GetActorOfClass` "/Game/TRPG/Tiles/Blueprints/BP_TileDataActor.BP_TileDataActor_C"))
  (set `self.TileData` _returnvalue))

(fn `SpawnUnitOnTile`
  (params (UnitData :type "/Game/TRPG/Units/SaveData/Struct_SaveUnitData Structure") (Tile :type "/Game/TRPG/Tiles/Blueprints/BP_GameTile Object Reference"))
  (bind (_unitname _characterstats _charactermaxstats _leveldata _weaponrankdata _items _skills _unitgameclass _ismandatorydeployment _combatstartingtile _movementtype _unitclass _appearancedata) (break `/Game/TRPG/Units/SaveData/Struct_SaveUnitData` UnitData))
  (bind _returnvalue (`|SpawnActorFromClass` _unitgameclass (`KismetMathLibrary.MakeTransform` (0.0 0.0 0.0)) "Undefined" "MultiplyWithRoot" (`GameplayStatics.GetPlayerController` 0) null))
  (`GameTile.SetUnitOnTile` Tile _returnvalue (`GameTile.StartingUnitDirection` Tile))
  (`/Game/TRPG/Units/Blueprints/BP_GameUnitBase.LoadSaveData` _returnvalue UnitData)
  (`/Game/TRPG/Units/Blueprints/BP_GameUnitBase.Update Unit Faction` _returnvalue (enumliteral `EUnitFaction` "PLAYER"))
  (`/Game/TRPG/Units/Blueprints/BP_GameUnitBase.UpdateAppearanceData` _returnvalue _appearancedata _unitclass))

(fn `SpawnUnitsOnTiles`
  (params (Units :type "Array of /Game/TRPG/Units/SaveData/Struct_SaveUnitData Structure"))
  (for (_array_element _array_index) (`self.PreBattleUnitList`)
    (bind _output (`|GetArrayItem` (`self.StartingTIles`) _array_index))
    (`/Engine/EditorBlueprintResources/StandardMacros.IsValid` _output
      (:`Is Valid`
        (bind _asbp_game_tile (cast `/Game/TRPG/Tiles/Blueprints/BP_GameTile` _output))
        (`self.SpawnUnitOnTile` _array_element _asbp_game_tile)))))