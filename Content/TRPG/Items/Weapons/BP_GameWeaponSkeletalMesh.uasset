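; BP_GameWeaponSkeletalMesh is a TRPG weapon Blueprint for weapons displayed with a skeletal mesh, extending a parent weapon class.
; Its InitializeDynamicMaterials override calls the parent, then rebuilds the DynamicMaterials array with a dynamic instance of each mesh material, applied back to its slot.
; AttachToUnit only forwards to the parent, and the event graph holds only disabled placeholder events.
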(fn `AttachToUnit`
  (params (GameUnit :type "/Game/TRPG/Units/Blueprints/BP_GameUnitBase Object Reference") (BoneName :type Name) (RelativeTransform :type "Transform Structure"))
  (`parent.AttachToUnit` GameUnit BoneName RelativeTransform))

(fn `InitializeDynamicMaterials`
  (bind _skeletalmesh (`self.SkeletalMesh`))
  (`parent.InitializeDynamicMaterials`)
  (`KismetArrayLibrary.Array_Clear` (`self.DynamicMaterials`))
  (for (_array_element _array_index) (`MeshComponent.GetMaterials` _skeletalmesh)
    (bind _returnvalue (`KismetMaterialLibrary.CreateDynamicMaterialInstance` _array_element))
    (`KismetArrayLibrary.Array_Add` (`self.DynamicMaterials`) _returnvalue)
    (`PrimitiveComponent.SetMaterial` _skeletalmesh _array_index _returnvalue)))

(fn `UserConstructionScript`
  (`parent.UserConstructionScript`))