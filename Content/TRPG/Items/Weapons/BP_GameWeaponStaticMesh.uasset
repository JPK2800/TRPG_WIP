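; Static mesh variant of a TRPG weapon, built on a parent weapon class that handles attaching it to a game unit.
; Overrides InitializeDynamicMaterials to clear the DynamicMaterials array, then create a dynamic instance of each WeaponMesh material, store it and apply it to the same slot.
; The construction script and AttachToUnit only call the parent, and the event graph holds no active logic.
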(fn `AttachToUnit`
  (params (GameUnit :type "/Game/TRPG/Units/Blueprints/BP_GameUnitBase Object Reference") (BoneName :type Name) (RelativeTransform :type "Transform Structure"))
  (`parent.AttachToUnit` GameUnit BoneName RelativeTransform))

(fn `InitializeDynamicMaterials`
  (bind _weaponmesh (`self.WeaponMesh`))
  (`parent.InitializeDynamicMaterials`)
  (`KismetArrayLibrary.Array_Clear` (`self.DynamicMaterials`))
  (for (_array_element _array_index) (`MeshComponent.GetMaterials` _weaponmesh)
    (bind _returnvalue (`KismetMaterialLibrary.CreateDynamicMaterialInstance` _array_element))
    (`KismetArrayLibrary.Array_Add` (`self.DynamicMaterials`) _returnvalue)
    (`PrimitiveComponent.SetMaterial` _weaponmesh _array_index _returnvalue)))

(fn `UserConstructionScript`
  (`parent.UserConstructionScript`))