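; Grid tile actor for the tactical RPG that shows navigable, attackable and interactable highlights plus a movement path arrow.
; BeginPlay binds to the tile's set and unset events, which toggle the matching overlay components.
; For routes, the origin and target cardinal directions select a no-movement, start, end, straight or turn arrow material and its world rotation.
; It also exposes its terrain type and per-movement-type terrain data lookup.
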(event `self.ReceiveBeginPlay`
  (add `self.OnTileSetNavigable` (delegate `OnTileSetNavigable_Event`))
  (add `self.OnTileUnsetNavigable` (delegate `OnTileUnsetNavigable_Event`))
  (add `self.OnTileSetAttackable` (delegate `OnTileSetAttackable_Event`))
  (add `self.OnTileUnsetAttackable` (delegate `OnTileUnsetAttackable_Event`))
  (add `self.OnTileSetInteractable` (delegate `OnTileSetInteractable_Event`))
  (add `self.OnTileUnsetInteractable` (delegate `OnTileUnsetInteractable_Event`))
  (add `self.OnTileSetRoutable` (delegate `OnTileSetRoutable_Event`))
  (add `self.OnTileUnsetRoutable` (delegate `OnTileUnsetRoutable_Event`)))

(event `OnTileUnsetNavigable_Event`
  (`self.SetNavigableTileVisibility` false))

(event `OnTileSetAttackable_Event`
  (`self.SetAttackableTileVisibility` true))

(event `OnTileUnsetAttackable_Event`
  (`self.SetAttackableTileVisibility` false))

(event `OnTileSetInteractable_Event`
  (`self.SetInteractableTileVisibility` true))

(event `OnTileUnsetInteractable_Event`
  (`self.SetInteractableTileVisibility` false))

(event `OnTileSetRoutable_Event` :!signature `self.OnTileSetRoutable`
  (params (OriginDirection :type "ECardinalDirections Enum" :default "NONE") (TargetDirection :type "ECardinalDirections Enum" :default "NONE"))
  (`self.SetArrowPathVisibility` true OriginDirection TargetDirection))

(event `OnTileUnsetRoutable_Event`
  (`self.SetArrowPathVisibility` false))

(event `OnTileSetNavigable_Event`
  (`self.SetNavigableTileVisibility` true))

(fn `GetTerrainInfoForUnit`
  (params (UnitMovementTypeInBytes :type Byte))
  (returns (ReturnValue :type "TerrainInfo Structure"))
  (return (`/Game/TRPG/Tiles/BlueprintFunctions/BPFL_DefaultTerrainData.GetTerrainDataForUnit` (cast `/Game/TRPG/Units/UnitData/EUnitMovementTypes` UnitMovementTypeInBytes) (`self.TileType`))))

(fn `GetTerrainTypeByte`
  (returns (ReturnValue :type Byte))
  (return (`self.TileType`)))

(fn `SetArrowPathVisibility`
  (params (Toggle :type Boolean) (Origin :type "ECardinalDirections Enum" :default "NONE") (Target :type "ECardinalDirections Enum" :default "NONE"))
  (locals (OriginByte :type Byte :default 0) (TargetByte :type Byte :default 0))
  (`|ExecutionSequence`
    (:`then_0`
      (`SceneComponent.SetHiddenInGame` (`self.Tile_ArrowPath`) (not Toggle) false))
    (:`then_1`
      (if Toggle
        (set `local.OriginByte` (`KismetSystemLibrary.MakeLiteralByte` Origin))
        (set `local.TargetByte` (`KismetSystemLibrary.MakeLiteralByte` Target))
        (`|ExecutionSequence`
          (:`then_0`
            ;[1 0.9823 0.6376] Is path beginning
            (if (== (`local.OriginByte`) (`KismetSystemLibrary.MakeLiteralByte` (enumliteral `ECardinalDirections` "NONE")))
              (if (== (`local.TargetByte`) (`KismetSystemLibrary.MakeLiteralByte` (enumliteral `ECardinalDirections` "NONE")))
                ;[1 1 1] Is both start and end tile
                (`PrimitiveComponent.SetMaterial` (`self.Tile_ArrowPath`) 0 "/Game/TRPG/Tiles/Materials/MI_PathNoMovement.MI_PathNoMovement")
                (return)
                (else
                  (`PrimitiveComponent.SetMaterial` (`self.Tile_ArrowPath`) 0 "/Game/TRPG/Tiles/Materials/MI_PathArrowStart.MI_PathArrowStart")
                  (`|ExecutionSequence`
                    (:`then_0`
                      (if (== (`local.TargetByte`) (`KismetSystemLibrary.MakeLiteralByte` (enumliteral `ECardinalDirections` "UP_DIR")))
                        (`SceneComponent.K2_SetWorldRotation` (`self.Tile_ArrowPath`) (struct :`Yaw` 90.0) false false)
                        (return)))
                    (:`then_1`
                      (if (== (`local.TargetByte`) (`KismetSystemLibrary.MakeLiteralByte` (enumliteral `ECardinalDirections` "RIGHT_DIR")))
                        (`SceneComponent.K2_SetWorldRotation` (`self.Tile_ArrowPath`) (struct :`Yaw` 180.0) false false)
                        (return)))
                    (:`then_2`
                      (if (== (`local.TargetByte`) (`KismetSystemLibrary.MakeLiteralByte` (enumliteral `ECardinalDirections` "DOWN_DIR")))
                        (`SceneComponent.K2_SetWorldRotation` (`self.Tile_ArrowPath`) (struct :`Yaw` -90.0) false false)
                        (return)))
                    (:`then_3`
                      (if (== (`local.TargetByte`) (`KismetSystemLibrary.MakeLiteralByte` (enumliteral `ECardinalDirections` "LEFT_DIR")))
                        (`SceneComponent.K2_SetWorldRotation` :`self` (`self.Tile_ArrowPath`))
                        (return))))))))
          (:`then_1`
            ;[1 0.9823 0.6376] Is path ending
            (if (== (`local.TargetByte`) (`KismetSystemLibrary.MakeLiteralByte` (enumliteral `ECardinalDirections` "NONE")))
              (`PrimitiveComponent.SetMaterial` (`self.Tile_ArrowPath`) 0 "/Game/TRPG/Tiles/Materials/MI_PathArrowEnd.MI_PathArrowEnd")
              (`|ExecutionSequence`
                (:`then_0`
                  (if (== (`local.OriginByte`) (`KismetSystemLibrary.MakeLiteralByte` (enumliteral `ECardinalDirections` "UP_DIR")))
                    (`SceneComponent.K2_SetWorldRotation` (`self.Tile_ArrowPath`) (struct :`Yaw` -90.0) false false)
                    (return)))
                (:`then_1`
                  (if (== (`local.OriginByte`) (`KismetSystemLibrary.MakeLiteralByte` (enumliteral `ECardinalDirections` "RIGHT_DIR")))
                    (`SceneComponent.K2_SetWorldRotation` :`self` (`self.Tile_ArrowPath`))
                    (return)))
                (:`then_2`
                  (if (== (`local.OriginByte`) (`KismetSystemLibrary.MakeLiteralByte` (enumliteral `ECardinalDirections` "DOWN_DIR")))
                    (`SceneComponent.K2_SetWorldRotation` (`self.Tile_ArrowPath`) (struct :`Yaw` 90.0) false false)
                    (return)))
                (:`then_3`
                  (if (== (`local.OriginByte`) (`KismetSystemLibrary.MakeLiteralByte` (enumliteral `ECardinalDirections` "LEFT_DIR")))
                    (`SceneComponent.K2_SetWorldRotation` (`self.Tile_ArrowPath`) (struct :`Yaw` 180.0) false false)
                    (return))))))
          (:`then_2`
            (`|ExecutionSequence`
              (:`then_0`
                ;[0.5089 0.1946 0.2346] Straight path north/south
                (if (or (and (== (`local.OriginByte`) (`KismetSystemLibrary.MakeLiteralByte` (enumliteral `ECardinalDirections` "DOWN_DIR"))) (== (`local.TargetByte`) (`KismetSystemLibrary.MakeLiteralByte` (enumliteral `ECardinalDirections` "UP_DIR")))) (and (== (`local.OriginByte`) (`KismetSystemLibrary.MakeLiteralByte` (enumliteral `ECardinalDirections` "UP_DIR"))) (== (`local.TargetByte`) (`KismetSystemLibrary.MakeLiteralByte` (enumliteral `ECardinalDirections` "DOWN_DIR")))))
                  (`PrimitiveComponent.SetMaterial` (`self.Tile_ArrowPath`) 0 "/Game/TRPG/Tiles/Materials/MI_PathArrowStraight.MI_PathArrowStraight")
                  (`SceneComponent.K2_SetWorldRotation` (`self.Tile_ArrowPath`) (struct :`Yaw` 90.0) false false)
                  (return)))
              (:`then_1`
                ;[0.5089 0.1946 0.2346] Straight path east/west
                (if (or (and (== (`local.OriginByte`) (`KismetSystemLibrary.MakeLiteralByte` (enumliteral `ECardinalDirections` "LEFT_DIR"))) (== (`local.TargetByte`) (`KismetSystemLibrary.MakeLiteralByte` (enumliteral `ECardinalDirections` "RIGHT_DIR")))) (and (== (`local.OriginByte`) (`KismetSystemLibrary.MakeLiteralByte` (enumliteral `ECardinalDirections` "RIGHT_DIR"))) (== (`local.TargetByte`) (`KismetSystemLibrary.MakeLiteralByte` (enumliteral `ECardinalDirections` "LEFT_DIR")))))
                  (`PrimitiveComponent.SetMaterial` (`self.Tile_ArrowPath`) 0 "/Game/TRPG/Tiles/Materials/MI_PathArrowStraight.MI_PathArrowStraight")
                  (`SceneComponent.K2_SetWorldRotation` :`self` (`self.Tile_ArrowPath`))
                  (return)))))
          (:`then_3`
            (`|ExecutionSequence`
              (:`then_0`
                ;[1 1 1] South-to-East
                (if (and (== (`local.OriginByte`) (`KismetSystemLibrary.MakeLiteralByte` (enumliteral `ECardinalDirections` "DOWN_DIR"))) (== (`local.TargetByte`) (`KismetSystemLibrary.MakeLiteralByte` (enumliteral `ECardinalDirections` "RIGHT_DIR"))))
                  (`PrimitiveComponent.SetMaterial` (`self.Tile_ArrowPath`) 0 "/Game/TRPG/Tiles/Materials/MI_PathArrowTurnRight.MI_PathArrowTurnRight")
                  (`SceneComponent.K2_SetWorldRotation` (`self.Tile_ArrowPath`) (struct :`Yaw` 90.0) false false)
                  (return)))
              (:`then_1`
                ;[1 1 1] East-to-North
                (if (and (== (`local.OriginByte`) (`KismetSystemLibrary.MakeLiteralByte` (enumliteral `ECardinalDirections` "RIGHT_DIR"))) (== (`local.TargetByte`) (`KismetSystemLibrary.MakeLiteralByte` (enumliteral `ECardinalDirections` "UP_DIR"))))
                  (`PrimitiveComponent.SetMaterial` (`self.Tile_ArrowPath`) 0 "/Game/TRPG/Tiles/Materials/MI_PathArrowTurnRight.MI_PathArrowTurnRight")
                  (`SceneComponent.K2_SetWorldRotation` :`self` (`self.Tile_ArrowPath`))
                  (return)))
              (:`then_2`
                ;[1 1 1] North-to-West
                (if (and (== (`local.OriginByte`) (`KismetSystemLibrary.MakeLiteralByte` (enumliteral `ECardinalDirections` "UP_DIR"))) (== (`local.TargetByte`) (`KismetSystemLibrary.MakeLiteralByte` (enumliteral `ECardinalDirections` "LEFT_DIR"))))
                  (`PrimitiveComponent.SetMaterial` (`self.Tile_ArrowPath`) 0 "/Game/TRPG/Tiles/Materials/MI_PathArrowTurnRight.MI_PathArrowTurnRight")
                  (`SceneComponent.K2_SetWorldRotation` (`self.Tile_ArrowPath`) (struct :`Yaw` -90.0) false false)
                  (return)))
              (:`then_3`
                ;[1 1 1] West-to-South
                (if (and (== (`local.OriginByte`) (`KismetSystemLibrary.MakeLiteralByte` (enumliteral `ECardinalDirections` "LEFT_DIR"))) (== (`local.TargetByte`) (`KismetSystemLibrary.MakeLiteralByte` (enumliteral `ECardinalDirections` "DOWN_DIR"))))
                  (`PrimitiveComponent.SetMaterial` (`self.Tile_ArrowPath`) 0 "/Game/TRPG/Tiles/Materials/MI_PathArrowTurnRight.MI_PathArrowTurnRight")
                  (`SceneComponent.K2_SetWorldRotation` (`self.Tile_ArrowPath`) (struct :`Yaw` 180.0) false false)
                  (return)))
              (:`then_4`
                ;[1 1 1] South-to-west
                (if (and (== (`local.OriginByte`) (`KismetSystemLibrary.MakeLiteralByte` (enumliteral `ECardinalDirections` "DOWN_DIR"))) (== (`local.TargetByte`) (`KismetSystemLibrary.MakeLiteralByte` (enumliteral `ECardinalDirections` "LEFT_DIR"))))
                  (`PrimitiveComponent.SetMaterial` (`self.Tile_ArrowPath`) 0 "/Game/TRPG/Tiles/Materials/MI_PathArrowTurnLeft.MI_PathArrowTurnLeft")
                  (`SceneComponent.K2_SetWorldRotation` (`self.Tile_ArrowPath`) (struct :`Yaw` 90.0) false false)
                  (return)))
              (:`then_5`
                ;[1 1 1] East-to-South
                (if (and (== (`local.OriginByte`) (`KismetSystemLibrary.MakeLiteralByte` (enumliteral `ECardinalDirections` "RIGHT_DIR"))) (== (`local.TargetByte`) (`KismetSystemLibrary.MakeLiteralByte` (enumliteral `ECardinalDirections` "DOWN_DIR"))))
                  (`PrimitiveComponent.SetMaterial` (`self.Tile_ArrowPath`) 0 "/Game/TRPG/Tiles/Materials/MI_PathArrowTurnLeft.MI_PathArrowTurnLeft")
                  (`SceneComponent.K2_SetWorldRotation` :`self` (`self.Tile_ArrowPath`))
                  (return)))
              (:`then_6`
                ;[1 1 1] North-to-East
                (if (and (== (`local.OriginByte`) (`KismetSystemLibrary.MakeLiteralByte` (enumliteral `ECardinalDirections` "UP_DIR"))) (== (`local.TargetByte`) (`KismetSystemLibrary.MakeLiteralByte` (enumliteral `ECardinalDirections` "RIGHT_DIR"))))
                  (`PrimitiveComponent.SetMaterial` (`self.Tile_ArrowPath`) 0 "/Game/TRPG/Tiles/Materials/MI_PathArrowTurnLeft.MI_PathArrowTurnLeft")
                  (`SceneComponent.K2_SetWorldRotation` (`self.Tile_ArrowPath`) (struct :`Yaw` -90.0) false false)
                  (return)))
              (:`then_7`
                ;[1 1 1] West-to-North
                (if (and (== (`local.OriginByte`) (`KismetSystemLibrary.MakeLiteralByte` (enumliteral `ECardinalDirections` "LEFT_DIR"))) (== (`local.TargetByte`) (`KismetSystemLibrary.MakeLiteralByte` (enumliteral `ECardinalDirections` "UP_DIR"))))
                  (`PrimitiveComponent.SetMaterial` (`self.Tile_ArrowPath`) 0 "/Game/TRPG/Tiles/Materials/MI_PathArrowTurnLeft.MI_PathArrowTurnLeft")
                  (`SceneComponent.K2_SetWorldRotation` (`self.Tile_ArrowPath`) (struct :`Yaw` 180.0) false false)
                  (return))))))))))

(fn `SetAttackableTileVisibility`
  (params (Toggle :type Boolean))
  (`SceneComponent.SetVisibility` (`self.Tile_Attackable`) Toggle false))

(fn `SetInteractableTileVisibility`
  (params (Toggle :type Boolean))
  (`SceneComponent.SetVisibility` (`self.Tile_Interactable`) Toggle false))

(fn `SetNavigableTileVisibility`
  (params (Toggle :type Boolean))
  (`SceneComponent.SetHiddenInGame` (`self.Tile_Navigable`) (not Toggle) false))

(fn `UserConstructionScript`)