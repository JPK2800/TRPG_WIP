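; Base status effect for the tactical RPG combat system, storing the afflicted unit and the unit that inflicted it.
; Turn start, turn end, turn update and trigger functions are empty hooks.
; A phase-change check returns true when the new phase matches the owner's faction, though the NPC case compares a constant 0 instead of that faction.
; Removal is delegated to the owner unit.
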(fn `InitStatus`
  (params (UnitWithStatus :type "/Game/TRPG/Units/Blueprints/BP_GameUnitBase Object Reference") (InflictingUnit :type "/Game/TRPG/Units/Blueprints/BP_GameUnitBase Object Reference"))
  (set `self.InstigatorUnit` InflictingUnit)
  (set `self.OwnerUnit` UnitWithStatus))

(fn `OnThisUnitTurnEnd`)

(fn `OnThisUnitTurnStart`)

(fn `RemoveObjectFromOwner`
  (`/Game/TRPG/Units/Blueprints/BP_GameUnitBase.RemoveStatusEffect` (`self.OwnerUnit`) self))

(fn `ShouldTriggerOnPhaseChange`
  (params (NewPhase :type "ECombatPhase Enum" :default "NO_PHASE"))
  (returns (ShouldTrigger :type Boolean))
  (bind _ownerunit (`self.OwnerUnit`))
  (bind _unitfaction (`GameUnit.UnitFaction` _ownerunit))
  (`|ExecutionSequence`
    (:`then_0`
      (`/Engine/EditorBlueprintResources/StandardMacros.IsValid` _ownerunit
        (:`Is Valid`
          (switch `ECombatPhase` NewPhase
            (:`PLAYER_PHASE`
              (if (== _unitfaction (`KismetSystemLibrary.MakeLiteralByte` (enumliteral `EUnitFaction` "PLAYER")))
                (return true)))
            (:`PARTNER_PHASE`
              (if (== _unitfaction (`KismetSystemLibrary.MakeLiteralByte` (enumliteral `EUnitFaction` "PARTNER")))
                (return true)))
            (:`ENEMY_PHASE`
              (if (== _unitfaction (`KismetSystemLibrary.MakeLiteralByte` (enumliteral `EUnitFaction` "ENEMY")))
                (return true)))
            (:`NPC_PHASE`
              (if (== 0 (`KismetSystemLibrary.MakeLiteralByte` (enumliteral `EUnitFaction` "NPC")))
                (return true)))))))
    (:`then_1`
      (return false))))

(fn `TriggerStatusEffect`)

(fn `UpdateCurrentTurn`)