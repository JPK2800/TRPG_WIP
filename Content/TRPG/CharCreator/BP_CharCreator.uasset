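; Character creator pawn that previews a customizable TRPG unit and is possessed by the player controller on BeginPlay.
; Head, hair, face and two class-misc meshes follow the body skeleton through leader pose.
; It creates the creator widget and binds its eye, horn, color and misc option events.
; Update functions edit the savable appearance struct, then reapply meshes and materials from GetUnitAppearances using one fixed unit class.
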(event `self.ReceiveBeginPlay`
  (`Controller.Possess` (`GameplayStatics.GetPlayerController` 0) self)
  (`|ExecutionSequence`
    (:`then_0`
      (`SkinnedMeshComponent.SetLeaderPoseComponent` (`self.HeadMesh`) (`self.SkeletalMesh`) false false)
      (`SkinnedMeshComponent.SetLeaderPoseComponent` (`self.HairMesh`) (`self.SkeletalMesh`) false false)
      (`SkinnedMeshComponent.SetLeaderPoseComponent` (`self.FaceMesh`) (`self.SkeletalMesh`) false false)
      (`SkinnedMeshComponent.SetLeaderPoseComponent` (`self.ClassMisc1`) (`self.SkeletalMesh`) false false)
      (`SkinnedMeshComponent.SetLeaderPoseComponent` (`self.ClassMisc2`) (`self.SkeletalMesh`) false false))
    (:`then_1`
      (`self.OnUpdateAppearance` (`self.AppearanceData`)))
    (:`then_2`
      (`self.InitWidget`))))

(fn `InitWidget`
  (bind _returnvalue (`|CreateWidget` "/Game/TRPG/CharCreator/WBP_CharCreatorWidget.WBP_CharCreatorWidget_C" (`GameplayStatics.GetPlayerController` 0)))
  (`/Game/TRPG/CharCreator/WBP_CharCreatorWidget.InitWidget` _returnvalue)
  (`UserWidget.AddToPlayerScreen` _returnvalue 0)
  (bind _output_get (set `self.CharWidget` _returnvalue))
  (add `/Game/TRPG/CharCreator/WBP_CharCreatorWidget.SetNewEyeOption` _output_get (`|CreateDelegate` :!event `UpdateEyes`))
  (add `/Game/TRPG/CharCreator/WBP_CharCreatorWidget.SetNewHornOption` _output_get (`|CreateDelegate` :!event `UpdateHorns`))
  (add `/Game/TRPG/CharCreator/WBP_CharCreatorWidget.SetNewColorOption` _output_get (`|CreateDelegate` :!event `UpdateColor`))
  (add `/Game/TRPG/CharCreator/WBP_CharCreatorWidget.SetNewMiscOption` _output_get (`|CreateDelegate` :!event `UpdateMisc`)))

(fn `OnUpdateAppearance`
  (params (SavableAppearance :type "/Game/TRPG/Units/SavableUnitAppearanceData/Struct_SavableUnitAppearanceData Structure"))
  (bind _skeletalmesh (`self.SkeletalMesh`))
  (bind _headmesh (`self.HeadMesh`))
  (bind _hairmesh (`self.HairMesh`))
  (bind _facemesh (`self.FaceMesh`))
  (bind _classmisc1 (`self.ClassMisc1`))
  (bind _classmisc2 (`self.ClassMisc2`))
  (bind (_bodytype _bodymesh _bodymaterials _headmesh_2 _headmaterials _hairmesh_2 _hairmaterials _facemesh_2 _facematerials _hairmaincolor _hairsecondarycolor _classmiscmesh1 _classmiscmesh2) (break `/Game/TRPG/Units/SavableUnitAppearanceData/Struct_UnitAppearanceData` (`/Game/TRPG/Units/SavableUnitAppearanceData/BPFL_GetUnitAppearances.GetUnitAppearances` SavableAppearance "NewEnumerator2")))
  (bind _output (`|GetArrayItem` _bodymaterials))
  (set `SkeletalMeshComponent.SkeletalMeshAsset` _bodymesh _skeletalmesh)
  (for _array_element _bodymaterials
    (`PrimitiveComponent.SetMaterial` _skeletalmesh 0 _array_element))
  (`SkeletalMeshComponent.SetSkeletalMeshAsset` _headmesh _headmesh_2)
  (for (_array_element_2 _array_index) _headmaterials
    (`PrimitiveComponent.SetMaterial` _headmesh _array_index _array_element_2))
  (`SkeletalMeshComponent.SetSkeletalMeshAsset` _hairmesh _hairmesh_2)
  (for (_array_element_3 _array_index_2) _hairmaterials
    (`PrimitiveComponent.SetMaterial` _hairmesh _array_index_2 _array_element_3))
  (`SkeletalMeshComponent.SetSkeletalMeshAsset` _facemesh _facemesh_2)
  (for (_array_element_4 _array_index_3) _facematerials
    (`PrimitiveComponent.SetMaterial` _facemesh _array_index_3 _array_element_4))
  (`SkeletalMeshComponent.SetSkeletalMeshAsset` _classmisc1 _classmiscmesh1)
  (`PrimitiveComponent.SetMaterial` _classmisc1 0 _output)
  (`SkeletalMeshComponent.SetSkeletalMeshAsset` _classmisc2 _classmiscmesh2)
  (`PrimitiveComponent.SetMaterial` _classmisc2 0 _output))

(fn `UpdateColor`
  (params (Color :type Byte))
  (bind _structout (setmembers `/Game/TRPG/Units/SavableUnitAppearanceData/Struct_SavableUnitAppearanceData` :`StructRef` (`self.AppearanceData`) :`CustomizationOption_A` Color))
  (`self.OnUpdateAppearance` _structout))

(fn `UpdateEyes`
  (params (Eye :type Byte))
  (bind _structout (setmembers `/Game/TRPG/Units/SavableUnitAppearanceData/Struct_SavableUnitAppearanceData` :`StructRef` (`self.AppearanceData`) :`CustomizationOption_C` Eye))
  (`self.OnUpdateAppearance` _structout))

(fn `UpdateHorns`
  (params (Horns :type Byte))
  (bind _structout (setmembers `/Game/TRPG/Units/SavableUnitAppearanceData/Struct_SavableUnitAppearanceData` :`StructRef` (`self.AppearanceData`) :`CustomizationOption_B` Horns))
  (`self.OnUpdateAppearance` _structout))

(fn `UpdateMisc`
  (params (Misc :type Byte))
  (bind _structout (setmembers `/Game/TRPG/Units/SavableUnitAppearanceData/Struct_SavableUnitAppearanceData` :`StructRef` (`self.AppearanceData`) :`CustomizationOption_D` Misc))
  (`self.OnUpdateAppearance` _structout))

(fn `UserConstructionScript`)