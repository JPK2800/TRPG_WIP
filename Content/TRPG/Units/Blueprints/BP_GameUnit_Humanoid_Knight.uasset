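; Knight variant of the humanoid TRPG game unit, adding a plate armor mesh to the base body.
; On BeginPlay the PlateArmor component takes BodyMesh as its leader pose component, so it follows the body animation.
; After the parent sets up dynamic materials, the armor's first material slot is set to the body's first material, so both share it.
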(event `self.ReceiveBeginPlay`
  (`parent.ReceiveBeginPlay`)
  (`SkinnedMeshComponent.SetLeaderPoseComponent` (`self.PlateArmor`) (`self.BodyMesh`) false false))

(fn `InitializeDynamicMaterials`
  (`parent.InitializeDynamicMaterials`)
  (`PrimitiveComponent.SetMaterial` (`self.PlateArmor`) 0 (`PrimitiveComponent.GetMaterial` (`self.BodyMesh`) 0)))

(fn `UserConstructionScript`
  (`parent.UserConstructionScript`))