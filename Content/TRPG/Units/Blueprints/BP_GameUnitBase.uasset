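; Base class for tactical RPG units, holding stats, HP, inventory, skills and movement type loaded from save data.
; Loading instantiates equipped skills and passes the equipped weapon to UpdateWeaponAnimations, an empty hook for child classes such as BP_GameUnit_3D.
; Tick moves the unit toward a target tile at constant speed, then signals arrival.
; Helpers reset per-turn actions and movement, clamp HP changes with notification, and report weapon range and targeting.
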(event `self.ReceiveBeginPlay`)

(event `self.ReceiveTick`
  (params (DeltaSeconds :type "Float (single-precision)"))
  (`self.MoveUnitToPositionStep` DeltaSeconds))

(event `self.ResetUnitMovementAndActions`
  (bind _unitstats_statmap (break `/Game/TRPG/CombatCalculations/Struct_Stats` (`self.UnitStats`)))
  (bind (_value _returnvalue) (`BlueprintMapLibrary.Map_Find` _unitstats_statmap "NewEnumerator9"))
  (`self.SetUnitRemainingActions` 1)
  (if _returnvalue
    (`self.SetUnitRemainingSpaces` _value)))

(event `self.MoveUnitToTile`
  (params (Tile :type "GameTile Object Reference"))
  (`self.MoveUnitToPositionStart` Tile))

(event `self.StopMovementToTiles`
  (`self.CancelMoveUnit`))

(fn `ApplyHpChange`
  (params (HpChange :type Integer))
  (bind _hpremaining (`self.HpRemaining`))
  (bind (_unitstats_statmap _unitstats_hp) (break `/Game/TRPG/CombatCalculations/Struct_Stats` (`self.UnitStats`)))
  (bind _returnvalue (`KismetMathLibrary.Clamp` (+ _hpremaining HpChange) 0 _unitstats_hp))
  ;[1 0.2753 0.498] Updates HP
  (`self.OnHpUpdate` _returnvalue _hpremaining)
  (set `self.HpRemaining` _returnvalue))

(fn `CancelMoveUnit`
  (set `self.DestLoc` (0.0 0.0 0.0))
  (set `self.DestTile` null)
  (set `self.MovingUnit` false))

(fn `GetEquippedItemOfType`
  (params (EquipmentSlotName :type String))
  (returns (ItemData :type "/Game/TRPG/Items/Struct_SaveItemData Structure") (FoundData :type Boolean) (WeaponType :type "/Game/TRPG/Items/Weapons/WeaponTypes/EWeaponTypes Enum") (WeaponActorClasses :type "Array of /Game/TRPG/Items/Weapons/BP_GameWeaponActor Class Reference"))
  ;[0.5573 0.1774 0.08251] Obtains the current equipped weapon data from UnitInventory
  (for _array_element (`self.UnitInventory`)
    (bind (_classtype _durability _isequipped) (break `/Game/TRPG/Items/Struct_SaveItemData` _array_element))
    (bind _asbp_equippable_weapon_item (castclass `/Game/TRPG/Items/Weapons/BP_EquippableWeaponItem` _classtype))
    (bind (_weaponactorclasses _weaponanimationtype _equipmentslotname) (defaults `Object` _asbp_equippable_weapon_item))
    (if (and _isequipped (== _equipmentslotname EquipmentSlotName))
      (return _array_element true _weaponanimationtype _weaponactorclasses)))
  (return (struct) false "NewEnumerator0"))

(fn `GetUnitEquippedWeaponRange`
  (returns (MinRange :type Byte) (MaxRange :type Byte) (TargetsEnemies :type Boolean) (TargetsAllies :type Boolean) (ReturnValue :type Boolean))
  (bind (_itemdata _founddata) (`self.GetEquippedItemOfType` "Weapon"))
  (if _founddata
    (bind _asbp_equippable_weapon_item (castclass `/Game/TRPG/Items/Weapons/BP_EquippableWeaponItem` (`.ClassType_4_03CD550D40B1B34E1D7F1593541C128C` (break `/Game/TRPG/Items/Struct_SaveItemData` _itemdata)))
      (:`then`
        (bind (_weaponattributes_rank _weaponattributes_durability _weaponattributes_power _weaponattributes_accuracy _weaponattributes_critchance _weaponattributes_critpower _weaponattributes_ignoretargetdefenses _weaponattributes_ignoretargetdefensesoncrit _weaponattributes_rangemin _weaponattributes_rangemax _weaponattributes_weight _weaponattributes_weaponexperience _weaponattributes_weaponexperiencetype _weaponattributes_gainweaponexperience _weaponattributes_targetenemy _weaponattributes_targetally) (break `/Game/TRPG/Items/Weapons/Struct_WeaponAttributes` (defaults `Object` _asbp_equippable_weapon_item)))
        (return _weaponattributes_rangemin _weaponattributes_rangemax _weaponattributes_targetenemy _weaponattributes_targetally true))
      (:`CastFailed`
        _)))
  (return 0 0 false false false))

(fn `GetUnitMovementTypeInBytes`
  (returns (ReturnValue :type Byte))
  (return (`self.UnitMovementType`)))

(fn `InitializeHP`
  ;[0.3646 0.3646 0.3646] Sets HP to the stat value at the start of battle
  (set `self.HpRemaining` (`.HP_42_2739A0784D08D212217227B30DFB1003` (break `/Game/TRPG/CombatCalculations/Struct_Stats` (`self.UnitStats`)))))

(fn `InitializeSkills`
  (params (Skills :type "Array of /Game/TRPG/Skills/Struct_SaveSkillData Structure"))
  ;[1 1 1] Instantiate EquippedSkills
  (bind _output_get (set `self.UnitSkills` Skills))
  (for _array_element _output_get
    (bind (_skillclass _isequipped) (break `/Game/TRPG/Skills/Struct_SaveSkillData` _array_element))
    (if _isequipped
      (bind _returnvalue (`|GenericCreateObject` _skillclass))
      (`/Engine/EditorBlueprintResources/StandardMacros.IsValid` _returnvalue
        (:`Is Valid`
          (`KismetArrayLibrary.Array_Add` (`self.EquippedSkills`) _returnvalue))))))

(fn `LoadSaveData`
  (params (UnitSaveData :type "/Game/TRPG/Units/UnitData/Struct_SaveUnitData Structure"))
  (bind (_itemdata _founddata _weapontype _weaponactorclasses) (`self.GetEquippedItemOfType` "Weapon"))
  (`|ExecutionSequence`
    (:`then_0`
      (set `self.UnitName` UnitSaveData_UnitName_3_1A1C59DB47E1F5BEBD5F21AB786DE165))
    (:`then_1`
      (set `self.UnitStats` UnitSaveData_CharacterStats_10_43F9610741184A2455CC6A9F202EA602)
      (`self.InitializeHP`))
    (:`then_2`
      (set `self.UnitStatCaps` UnitSaveData_CharacterMaxStats_12_ABC1FBFE4F2258A0D759E1817A8E7AFB))
    (:`then_3`
      (set `self.UnitLevelData` UnitSaveData_LevelData_15_E6A0D1734E4600DB79CCF683D7F016C3))
    (:`then_4`
      (set `self.UnitWeaponRanks` UnitSaveData_WeaponRankData_18_0218DA364C4FBF536A403894EE872976))
    (:`then_5`
      (set `self.UnitInventory` UnitSaveData_Items_22_1ECB0D2A4BC629D66E77ADBD10C698CE))
    (:`then_6`
      (`self.InitializeSkills` UnitSaveData_Skills_29_AFF341CC4142C3F524D5A09936D851DB))
    (:`then_7`
      (if _founddata
        (`self.UpdateWeaponAnimations` _weapontype _weaponactorclasses)))
    (:`then_8`
      (set `self.UnitMovementType` UnitSaveData_MovementType_40_90834D26408B009732CA8F979EAC1989))))

(fn `MoveUnitToPositionEnd`
  (`self.K2_SetActorLocation` (`self.DestLoc`))
  (set `self.DestLoc` (0.0 0.0 0.0))
  (set `self.MovingUnit` false)
  (`self.OnTraveledToTile` (`self.DestTile`)))

(fn `MoveUnitToPositionStart`
  (params (TargetTile :type "GameTile Object Reference"))
  (bind _asbp_game_tile (cast `/Game/TRPG/Tiles/Blueprints/BP_GameTile` TargetTile))
  (set `self.DestLoc` (`SceneComponent.K2_GetComponentLocation` (`GameTile.UnitPositionComponent` _asbp_game_tile)))
  (set `self.MovingUnit` true)
  (set `self.DestTile` _asbp_game_tile))

(fn `MoveUnitToPositionStep`
  (params (DeltaTime :type "Float (double-precision)"))
  (bind _destloc (`self.DestLoc`))
  (bind _returnvalue (`KismetMathLibrary.VInterpTo_Constant` (`self.K2_GetActorLocation`) _destloc DeltaTime 650.0))
  (if (`self.MovingUnit`)
    (`self.K2_SetActorLocation` _returnvalue)
    (if (< (`KismetMathLibrary.Vector_Distance` _destloc _returnvalue) 2.0)
      (`self.MoveUnitToPositionEnd`))))

(fn `UpdateWeaponAnimations`
  (params (WeaponType :type "/Game/TRPG/Items/Weapons/WeaponTypes/EWeaponTypes Enum" :default "NewEnumerator0") (WeaponActorClasses :type "Array of /Game/TRPG/Items/Weapons/BP_GameWeaponActor Class Reference"))
  ;[1 1 1] Implement in child classes. BP_GameUnit_3D has an override to commucate this info to the animation blueprint.
)

(fn `UserConstructionScript`)