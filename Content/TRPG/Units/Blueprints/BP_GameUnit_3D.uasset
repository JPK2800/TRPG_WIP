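; 3D TRPG unit Blueprint that renders a character from modular body, head, face and hair meshes and attached weapons.
; Head, face and hair follow the body through leader pose, while appearance updates swap meshes and materials by save data and unit class.
; Weapon updates notify the body's AnimBP via IUnitAnimations and respawn weapon actors on attach bones.
; Dynamic material instances, rebuilt after appearance changes, let SetUnitGray grey out the unit and its weapons.
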(event `self.ReceiveBeginPlay`
  (`parent.ReceiveBeginPlay`)
  (`SkinnedMeshComponent.SetLeaderPoseComponent` (`self.HeadMesh`) (`self.BodyMesh`) false false)
  (`SkinnedMeshComponent.SetLeaderPoseComponent` (`self.FaceMesh`) (`self.BodyMesh`) false false)
  (`SkinnedMeshComponent.SetLeaderPoseComponent` (`self.HairMesh`) (`self.BodyMesh`) false false)
  (`self.InitializeDynamicMaterials`))

(event `self.SetUnitGray`
  (params (Toggle :type Boolean))
  (`self.ToggleGrayForMaterials` Toggle))

(fn `InitializeDynamicMaterials`
  (bind _bodymesh (`self.BodyMesh`))
  (bind _headmesh (`self.HeadMesh`))
  (bind _hairmesh (`self.HairMesh`))
  (bind _facemesh (`self.FaceMesh`))
  (`KismetArrayLibrary.Array_Clear` (`self.DynamicMaterials`))
  (`|ExecutionSequence`
    (:`then_0`
      (for (_array_element _array_index) (`MeshComponent.GetMaterials` _bodymesh)
        (bind _returnvalue (`KismetMaterialLibrary.CreateDynamicMaterialInstance` _array_element))
        (`KismetArrayLibrary.Array_Add` (`self.DynamicMaterials`) _returnvalue)
        (`PrimitiveComponent.SetMaterial` _bodymesh _array_index _returnvalue)))
    (:`then_1`
      (for (_array_element_2 _array_index_2) (`MeshComponent.GetMaterials` _headmesh)
        (bind _returnvalue_2 (`KismetMaterialLibrary.CreateDynamicMaterialInstance` _array_element_2))
        (`KismetArrayLibrary.Array_Add` (`self.DynamicMaterials`) _returnvalue_2)
        (`PrimitiveComponent.SetMaterial` _headmesh _array_index_2 _returnvalue_2)))
    (:`then_2`
      (for (_array_element_3 _array_index_3) (`MeshComponent.GetMaterials` _hairmesh)
        (bind _returnvalue_3 (`KismetMaterialLibrary.CreateDynamicMaterialInstance` _array_element_3))
        (`KismetArrayLibrary.Array_Add` (`self.DynamicMaterials`) _returnvalue_3)
        (`PrimitiveComponent.SetMaterial` _hairmesh _array_index_3 _returnvalue_3)))
    (:`then_3`
      (for (_array_element_4 _array_index_4) (`MeshComponent.GetMaterials` _facemesh)
        (bind _returnvalue_4 (`KismetMaterialLibrary.CreateDynamicMaterialInstance` _array_element_4))
        (`KismetArrayLibrary.Array_Add` (`self.DynamicMaterials`) _returnvalue_4)
        (`PrimitiveComponent.SetMaterial` _facemesh _array_index_4 _returnvalue_4)))))

(fn `ToggleGrayForMaterials`
  (params (Toggle :type Boolean))
  ;[1 1 1] Update the grayscale for weapons
  (`|ExecutionSequence`
    (:`then_0`
      (for _array_element (`self.WeaponActors`)
        (`/Game/TRPG/Items/Weapons/BP_GameWeaponActor.ToggleGray` _array_element Toggle)))
    (:`then_1`
      ;[1 1 1] Update the grayscale for this unit's meshes
      (for _array_element_2 (`self.DynamicMaterials`)
        (`MaterialInstanceDynamic.SetScalarParameterValue` _array_element_2 "IsGray" (`KismetMathLibrary.Conv_BoolToDouble` Toggle))))))

(fn `UpdateAppearanceData`
  (params (AppearanceSaveData :type "/Game/TRPG/Units/UnitAppearanceData/Struct_SavableUnitAppearanceData Structure") (UnitClass :type "/Game/TRPG/Units/UnitClasses/Enum_UnitClasses Enum" :default "NewEnumerator0"))
  (bind _bodymesh (`self.BodyMesh`))
  (bind _headmesh (`self.HeadMesh`))
  (bind _facemesh (`self.FaceMesh`))
  (bind _hairmesh (`self.HairMesh`))
  (bind (_bodytype _bodymesh_2 _bodymaterials _headmesh_2 _headmaterials _hairmesh_2 _hairmaterials _facemesh_2 _facematerials) (break `/Game/TRPG/Units/UnitAppearanceData/Struct_UnitAppearanceData` (`/Game/TRPG/Units/UnitAppearanceData/BPFL_GetUnitAppearances.GetUnitAppearances` AppearanceSaveData UnitClass)))
  (`parent.UpdateAppearanceData` AppearanceSaveData UnitClass)
  (`|ExecutionSequence`
    (:`then_0`
      (`SkeletalMeshComponent.SetSkeletalMeshAsset` _bodymesh _bodymesh_2)
      (for (_array_element _array_index) _bodymaterials
        (`PrimitiveComponent.SetMaterial` _bodymesh _array_index _array_element))
      (`SkeletalMeshComponent.SetSkeletalMeshAsset` _headmesh _headmesh_2)
      (for (_array_element_2 _array_index_2) _headmaterials
        (`PrimitiveComponent.SetMaterial` _headmesh _array_index_2 _array_element_2))
      (`SkeletalMeshComponent.SetSkeletalMeshAsset` _facemesh _facemesh_2)
      (for (_array_element_3 _array_index_3) _facematerials
        (`PrimitiveComponent.SetMaterial` _facemesh _array_index_3 _array_element_3))
      (`SkeletalMeshComponent.SetSkeletalMeshAsset` _hairmesh _hairmesh_2)
      (for (_array_element_4 _array_index_4) _hairmaterials
        (`PrimitiveComponent.SetMaterial` _hairmesh _array_index_4 _array_element_4)))
    (:`then_1`
      (`self.InitializeDynamicMaterials`))))

(fn `UpdateWeaponAnimations`
  (params (WeaponType :type "/Game/TRPG/Items/Weapons/WeaponTypes/EWeaponTypes Enum" :default "NewEnumerator0") (WeaponActorClasses :type "Array of /Game/TRPG/Items/Weapons/BP_GameWeaponActor Class Reference (by ref)"))
  (bind _bodymesh (`self.BodyMesh`))
  (bind _weaponattachbones (`self.WeaponAttachBones`))
  (bind _returnvalue (`SkeletalMeshComponent.GetAnimInstance` _bodymesh))
  (`parent.UpdateWeaponAnimations` WeaponType WeaponActorClasses)
  (`|ExecutionSequence`
    (:`then_0`
      ;[1 1 1] Update animations to anim blueprint using the IUnitAnimations interface.
      (if (`KismetSystemLibrary.DoesImplementInterface` _returnvalue "/Script/TRPG.IUnitAnimations")
        (message `IUnitAnimations.SetNewEquipWeaponType` _returnvalue WeaponType (`SkeletalMeshComponent.GetSkeletalMeshAsset` _bodymesh))))
    (:`then_1`
      ;[1 1 1] Destroy old weapons if any exist
      (for _array_element (`self.WeaponActors`)
        (`self.K2_DestroyActor` _array_element)))
    (:`then_2`
      ;[1 1 1] Spawn and attach new weapon actors
      (for (_array_element_2 _array_index) WeaponActorClasses
        (if (`KismetArrayLibrary.Array_IsValidIndex` _weaponattachbones _array_index)
          (bind _returnvalue_2 (`|SpawnActorFromClass` _array_element_2 (`KismetMathLibrary.MakeTransform` (0.0 0.0 0.0)) "Undefined" "MultiplyWithRoot" self null))
          (`self.K2_AttachToComponent` _returnvalue_2 (`self.BodyMesh`) (`|GetArrayItem` _weaponattachbones _array_index) "KeepRelative" "KeepRelative" "KeepWorld" true)
          (`KismetArrayLibrary.Array_Add` (`self.WeaponActors`) _returnvalue_2))))))

(fn `UserConstructionScript`
  (`parent.UserConstructionScript`))