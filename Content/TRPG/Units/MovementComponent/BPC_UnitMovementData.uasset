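; BPC_UnitMovementData is a unit component that builds per-terrain movement data for a tactical RPG unit.
; On BeginPlay, or through its InitializeMovementMap event, it casts its owner to BP_GameUnitBase.
; It loops over every default terrain type, looking up terrain data for the unit's movement type.
; The resulting terrain-to-data map is passed to SetMovementMap.
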(event `self.ReceiveBeginPlay`
  (`self.InitializeMovementMap`))

(event `self.InitializeMovementMap`
  (`self.InitMovementMap`))

(fn `InitMovementMap`
  (locals (TerrainDataMap :type "Map of Byte to TerrainInfo Structure"))
  (bind _asbp_game_unit (cast `/Game/TRPG/Units/Blueprints/BP_GameUnitBase` (`self.GetOwner`)))
  (for _index (range (enumcount `/Game/TRPG/Tiles/Blueprints/EDefaultTerrainTypes`))
    (bind _returnvalue (cast `/Game/TRPG/Tiles/Blueprints/EDefaultTerrainTypes` (`KismetMathLibrary.Conv_IntToByte` _index)))
    (`BlueprintMapLibrary.Map_Add` (`local.TerrainDataMap`) _returnvalue (`/Game/TRPG/Tiles/BlueprintFunctions/BPFL_DefaultTerrainData.GetTerrainDataForUnit` (`/Game/TRPG/Units/Blueprints/BP_GameUnitBase.UnitMovementType` _asbp_game_unit) _returnvalue)))
  (`self.SetMovementMap` (`local.TerrainDataMap`)))